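; Game mode that holds shared references to world managers and provides a rarity-to-color lookup for item display.
; On BeginPlay it finds and caches the dropped items manager and placeable objects manager actors in the level.
; GetColorByRarityEnum maps each rarity tier, from Useless to Special, to a fixed Slate color.
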(event EventBeginPlay
  (bind _returnvalue (Actor|GetActorOfClass "/Game/Blueprints/Singletones/BP_DroppedItemsManager.BP_DroppedItemsManager_C"))
  (Variables|Default|SetDroppedItemsManager _returnvalue)
  (bind _returnvalue_2 (Actor|GetActorOfClass "/Game/Blueprints/Singletones/BP_PlaceablesManager.BP_PlaceablesManager_C"))
  (Variables|Default|SetPlaceableObjectsManager _returnvalue_2))

(event EventTick
  (params (DeltaSeconds :type Float%20%28single-precision%29)))

(fn ConstructionScript)

(fn GetColorbyRarityEnum
  (params (Rarity :type EN_ItemRarity%20Enum :default "NewEnumerator0"))
  (switch Utilities|FlowControl|Switch|SwitchonEN_ItemRarity Rarity
    (:NewEnumerator0
      (return (Utilities|Struct|MakeSlateColor "(R=0.200000,G=0.200000,B=0.200000,A=1.000000)")))
    (:NewEnumerator1
      (return (Utilities|Struct|MakeSlateColor "(R=1.000000,G=1.000000,B=1.000000,A=1.000000)")))
    (:NewEnumerator2
      (return (Utilities|Struct|MakeSlateColor "(R=0.000000,G=0.600000,B=0.000000,A=1.000000)")))
    (:NewEnumerator3
      (return (Utilities|Struct|MakeSlateColor "(R=0.000000,G=0.200000,B=0.800000,A=1.000000)")))
    (:NewEnumerator4
      (return (Utilities|Struct|MakeSlateColor "(R=0.360784,G=0.000000,B=0.600000,A=1.000000)")))
    (:NewEnumerator5
      (return (Utilities|Struct|MakeSlateColor "(R=0.701961,G=0.000000,B=0.000000,A=1.000000)")))
    (:NewEnumerator6
      (return (Utilities|Struct|MakeSlateColor "(R=0.701961,G=0.701961,B=0.000000,A=1.000000)")))
    (:NewEnumerator7
      (return (Utilities|Struct|MakeSlateColor "(R=0.701961,G=0.211765,B=0.698039,A=1.000000)")))))