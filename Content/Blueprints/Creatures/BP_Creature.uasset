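; BP_Creature is a creature Blueprint with health, a health bar widget and a contact-damage attack against players.
; BeginPlay binds BPHealthComponent to the health bar widget and refreshes it.
; Attack applies ContactDamage to the health component of each BP_PlayerCharacter overlapping ContactDamageCollision, while StopAttacking clears the IsAttackLooped flag.
; On Destroyed, it runs the empty OnDie hook, then calls OnDeath.
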(event Custom|Attack
  (for _array_element (Collision|GetOverlappingActors (Variables|Default|GetContactDamageCollision) "/Game/Blueprints/Player/BP_PlayerCharacter.BP_PlayerCharacter_C" :!class /Script/Engine.PrimitiveComponent)
    (bind _asbp_player_character (Utilities|Casting|CastToBP_PlayerCharacter _array_element))
    (Default|TakeDamage (Variables|/Game/Blueprints/Player/BP_PlayerCharacter.BP_PlayerCharacter_C|GetBP_HealthComponent _asbp_player_character) (Variables|Default|GetContactDamage))))

(event EventBeginPlay
  (bind _wb_healthbar (Variables|Default|GetWB_HealthBar))
  (bind _returnvalue (UserInterface|GetWidget _wb_healthbar))
  (bind _aswb_creature_healt_bar (Utilities|Casting|CastToWB_CreatureHealtBar _returnvalue))
  (Default|SetHealthComponent _aswb_creature_healt_bar (Variables|Default|GetBP_HealthComponent))
  (Default|Update _aswb_creature_healt_bar))

(event EventDestroyed
  (CallFunction|OnDie)
  (Default|CallOnDeath))

(fn ConstructionScript)

(fn OnDie)

(fn StopAttacking
  (Variables|Default|SetIsAttackLooped false))