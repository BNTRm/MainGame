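; BP_AttackComponent is a creature component that handles melee weapon hit detection and damage.
; SetWeaponSMComponentAndDamage caches the held weapon's static mesh and damage value.
; MeleeTrace runs a debug-drawn capsule trace for pawns using the mesh's BottomSocket and TopSocket, ignoring the owner.
; A hit player character or creature takes that damage through its health component.
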(event EventBeginPlay)

(event EventTick
  (params (DeltaSeconds :type Float%20%28single-precision%29)))

(fn MeleeTrace
  (bind _weaponsmcomponent (Variables|Default|GetWeaponSMComponent))
  (bind _damage (Variables|Default|GetDamage))
  (bind _outhit (Class|KismetSystemLibrary|CapsuleTraceSingleforObjects (Transformation|GetSocketLocation _weaponsmcomponent "BottomSocket") (Transformation|GetSocketLocation _weaponsmcomponent "TopSocket") 4.0 4.0 (Utilities|Array|MakeArray "ObjectTypeQuery3") false (Utilities|Array|MakeArray (Components|GetOwner)) "ForDuration" true "(R=1.000000,G=0.000000,B=0.000000,A=1.000000)" "(R=0.000000,G=1.000000,B=0.000000,A=1.000000)" 0.1))
  (Utilities|FlowControl|Sequence
    (:then_0
      (bind _asbp_player_character (Utilities|Casting|CastToBP_PlayerCharacter (.HitActor (Collision|BreakHitResult _outhit))))
      (Default|TakeDamage (Variables|/Game/Blueprints/Player/BP_PlayerCharacter.BP_PlayerCharacter_C|GetBP_HealthComponent _asbp_player_character) _damage))
    (:then_1
      (bind _asbp_creature (Utilities|Casting|CastToBP_Creature (.HitActor (Collision|BreakHitResult _outhit))))
      (Default|TakeDamage (Variables|/Game/Blueprints/Creatures/BP_Creature.BP_Creature_C|GetBP_HealthComponent _asbp_creature) _damage))))

(fn SetWeaponSMComponentandDamage
  (params (WeaponInHands :type BP%20Item%20in%20Hands%20Object%20Reference) (Damage :type Integer))
  (Variables|Default|SetDamage Damage)
  (Variables|Default|SetWeaponSMComponent (Variables|/Game/Blueprints/Items/BP_Item_InHands.BP_Item_InHands_C|GetStaticMesh WeaponInHands)))