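; BP_DropComponent is a creature component that handles coin loot drops.
; On BeginPlay it binds to the owning BP_Creature's OnDeath event.
; Drop asks the level's BP_DroppedItemsManager to spawn copper and gold coins at the creature's capsule location, using configurable min/max ranges.
; The above-zero check and spawned quantity use separate random evaluations, so they can differ.
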(event EventBeginPlay
  (bind _output_get (Variables|Default|SetOwnerCreature (.AsBP%20Creature (Utilities|Casting|CastToBP_Creature (Components|GetOwner)))))
  (EventDispatchers|BindEventtoOnDeath _output_get (EventDispatchers|CreateEvent :!event Drop)))

(fn Drop
  (bind _coppercoins (Variables|Default|GetCopperCoins))
  (bind _goldcoins (Variables|Default|GetGoldCoins))
  (bind _returnvalue (Math|Random|RandomIntegerinRange (.min _goldcoins) (.max _goldcoins)))
  (bind _returnvalue_2 (Math|Random|RandomIntegerinRange (.min _coppercoins) (.max _coppercoins)))
  (LocalVariables|SetL_Location (Transformation|GetWorldLocation (Variables|/Script/Engine.Character|GetCapsuleComponent (Variables|Default|GetOwnerCreature))))
  (bind _returnvalue_3 (Actor|GetActorOfClass "/Game/Blueprints/Singletones/BP_DroppedItemsManager.BP_DroppedItemsManager_C"))
  (bind _output_get (LocalVariables|SetL_DroppedItemsManager _returnvalue_3))
  (Utilities|FlowControl|Sequence
    (:then_0
      (if (> _returnvalue_2 0)
        (Default|SpawnDroppedItem _output_get (LocalVariables|GetL_Location) "coin_copper" _returnvalue_2 "0, 0, 0")))
    (:then_1
      (if (> _returnvalue 0)
        (Default|SpawnDroppedItem _output_get (LocalVariables|GetL_Location) "coin_gold" _returnvalue "0, 0, 0")))))