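; BP_PurseComponent is a creature component that stores separate copper and gold coin counts, each with its own maximum.
; TakeCopperCoins and TakeGoldCoins add coins to the purse, clamp the total at that maximum and return the overflow that did not fit.
; Both functions fire the OnCoinsTaken dispatcher after every call, and the component uses no BeginPlay or Tick logic.
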(event EventBeginPlay)

(event EventTick
  (params (DeltaSeconds :type Float%20%28single-precision%29)))

(fn TakeCopperCoins
  (params (Count :type Integer))
  (bind _maxcoppercoins (Variables|Default|GetMaxCopperCoins))
  (bind _output_get (Variables|Default|SetCopperCoins (+ (Variables|Default|GetCopperCoins) Count)))
  (if (> _output_get (Variables|Default|GetMaxCopperCoins))
    (LocalVariables|SetL_Remain (- (Variables|Default|GetCopperCoins) _maxcoppercoins))
    (Variables|Default|SetCopperCoins _maxcoppercoins))
  (Default|CallOnCoinsTaken)
  (return (LocalVariables|GetL_Remain)))

(fn TakeGoldCoins
  (params (Count :type Integer))
  (bind _maxgoldcoins (Variables|Default|GetMaxGoldCoins))
  (bind _output_get (Variables|Default|SetGoldCoins (+ (Variables|Default|GetGoldCoins) Count)))
  (if (> _output_get (Variables|Default|GetMaxGoldCoins))
    (LocalVariables|SetL_Remain (- (Variables|Default|GetGoldCoins) _maxgoldcoins))
    (Variables|Default|SetGoldCoins _maxgoldcoins))
  (Default|CallOnCoinsTaken)
  (return (LocalVariables|GetL_Remain)))