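; Slot-based inventory component for player characters and storage actors, holding items in a fixed-size array of slot structs.
; Adding fills matching stacks one unit at a time up to the DT_Items max stack, then uses empty slots.
; Slot transfers run through a server event and swap or merge stacks, with multicast updates firing OnInventoryUpdated.
; Quick transfer moves a slot between the player and opened storage, choosing direction by owner type.
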(event Custom|MC_Update
  (Default|CallOnInventoryUpdated))

(event Custom|Server_TransferSlots
  (params (SourceIndex :type Integer) (SourceInventory :type BP%20Inventory%20Component%20Object%20Reference) (DestinationIndex :type Integer))
  (CallFunction|TransferSlots SourceIndex SourceInventory DestinationIndex))

(event EventBeginPlay
  (Utilities|Array|Resize (Variables|Default|GetItems) (Variables|Default|GetSize)))

(fn AddItem
  (params (ItemSlotStruct :type S%20Slot%20Item%20Structure))
  (LocalVariables|SetL_QuantityRemaining (.quantity ItemSlotStruct))
  (while (and (> (LocalVariables|GetL_QuantityRemaining) 0) (not (LocalVariables|GetL_IsFailed)))
    (bind (_index _isslotfound) (CallFunction|FindFirstSlotbyItemID (.itemid ItemSlotStruct)))
    (if _isslotfound
      (CallFunction|AddtoStack _index 1)
      (Math|Integer|DecrementInt (LocalVariables|GetL_QuantityRemaining))
      (elif (.HasEmptySlot (CallFunction|AnyEmptySlotsAvailable))
        (bind _success (CallFunction|CreateNewStack (Utilities|Struct|MakeS_SlotItem (.itemid ItemSlotStruct) 1 (.shielditemid ItemSlotStruct))))
        (if _success
          (Math|Integer|DecrementInt (LocalVariables|GetL_QuantityRemaining))
          (else
            (LocalVariables|SetL_IsFailed true)))
        (else
          (LocalVariables|SetL_IsFailed true)))))
  (return (not (LocalVariables|GetL_IsFailed)) (LocalVariables|GetL_QuantityRemaining)))

(fn AddtoStack
  (params (Index :type Integer) (Quantity :type Integer))
  (bind _items (Variables|Default|GetItems))
  (bind _output (Utilities|Array|Get(acopy) _items Index))
  (Utilities|Array|SetArrayElem (Variables|Default|GetItems) Index (Utilities|Struct|MakeS_SlotItem (.itemid _output) (+ (.quantity _output) Quantity) "None")))

(fn AnyEmptySlotsAvailable
  (for (_array_element _array_index) (Variables|Default|GetItems)
    (if (== (.Quantity (Utilities|Struct|BreakS_SlotItem _array_element)) 0)
      (return true _array_index)))
  (return false -1))

(fn CreateNewStack
  (params (ItemSlotStruct :type S%20Slot%20Item%20Structure))
  (bind (_hasemptyslot _emptyslotindex) (CallFunction|AnyEmptySlotsAvailable))
  (if _hasemptyslot
    (Utilities|Array|SetArrayElem (Variables|Default|GetItems) _emptyslotindex ItemSlotStruct)
    (return true)
    (else
      (return false))))

(fn FindFirstSlotbyItemID
  (params (ItemID :type Name))
  (for (_array_element _array_index) (Variables|Default|GetItems)
    (if (== (.ItemId (Utilities|Struct|BreakS_SlotItem _array_element)) ItemID)
      (if (< (.Quantity (Utilities|Struct|BreakS_SlotItem _array_element)) (CallFunction|GetItemMaxStack ItemID))
        (return _array_index true))))
  (return -1 false))

(fn GetItemMaxStack
  (params (ItemID :type Name))
  (bind _returnvalue (Utilities|GetDataTableRow "/Game/MAIN_GAME/Data/Items/DT_Items.DT_Items" ItemID)
    (:then
      (return (.maxstack _returnvalue)))
    (:RowNotFound
      (return -1))))

(fn GetSlotItemStructbyIndex
  (params (Index :type Integer))
  (return (Utilities|Array|Get(acopy) (Variables|Default|GetItems) Index)))

(fn SubtractfromStack
  (params (Index :type Integer) (Quantity :type Integer))
  (bind _items (Variables|Default|GetItems))
  (bind _items_2 (Variables|Default|GetItems))
  (bind _output (Utilities|Array|Get(acopy) _items_2 Index))
  (bind _returnvalue (- (.quantity _output) Quantity))
  (if (> _returnvalue 0)
    (Utilities|Array|SetArrayElem _items Index (Utilities|Struct|MakeS_SlotItem (.itemid _output) _returnvalue (.shielditemid _output)))
    (else
      (Utilities|Array|SetArrayElem _items Index (Utilities|Struct|MakeS_SlotItem "None" 0 "None"))))
  (CallFunction|MCUpdate))

(fn TransferSlots
  (params (SourceIndex :type Integer) (SourceInventory :type BP%20Inventory%20Component%20Object%20Reference) (DestinationIndex :type Integer))
  (LocalVariables|SetL_SourceSlotContent (Utilities|Array|Get(acopy) (Variables|BP_InventoryComponent_C|GetItems SourceInventory) SourceIndex))
  (if (not (< DestinationIndex 0))
    (if (!= (.itemid (LocalVariables|GetL_SourceSlotContent)) (.itemid (Utilities|Array|Get(acopy) (Variables|Default|GetItems) DestinationIndex)))
      ;[1 1 1] Swap (Different Items or empty)
      (Utilities|Array|SetArrayElem (Variables|BP_InventoryComponent_C|GetItems SourceInventory) SourceIndex (Utilities|Array|Get(acopy) (Variables|Default|GetItems) DestinationIndex))
      (Utilities|Array|SetArrayElem (Variables|Default|GetItems) DestinationIndex (LocalVariables|GetL_SourceSlotContent))
      (else
        ;[1 1 1] Stack (Same Items)
        (Utilities|Array|SetArrayElem (Variables|BP_InventoryComponent_C|GetItems SourceInventory) SourceIndex (Utilities|Struct|MakeS_SlotItem (select (> (Math|Integer|Clamp(Integer) (- (+ (.quantity (LocalVariables|GetL_SourceSlotContent)) (.quantity (Utilities|Array|Get(acopy) (Variables|Default|GetItems) DestinationIndex))) (CallFunction|GetItemMaxStack (.itemid (LocalVariables|GetL_SourceSlotContent)))) 0 (CallFunction|GetItemMaxStack (.itemid (LocalVariables|GetL_SourceSlotContent)))) 0) (.itemid (LocalVariables|GetL_SourceSlotContent)) "None") (Math|Integer|Clamp(Integer) (- (+ (.quantity (LocalVariables|GetL_SourceSlotContent)) (.quantity (Utilities|Array|Get(acopy) (Variables|Default|GetItems) DestinationIndex))) (CallFunction|GetItemMaxStack (.itemid (LocalVariables|GetL_SourceSlotContent)))) 0 (CallFunction|GetItemMaxStack (.itemid (LocalVariables|GetL_SourceSlotContent)))) "None"))
        (Utilities|Array|SetArrayElem (Variables|Default|GetItems) DestinationIndex (Utilities|Struct|MakeS_SlotItem (.itemid (LocalVariables|GetL_SourceSlotContent)) (Math|Integer|Clamp(Integer) (+ (.quantity (LocalVariables|GetL_SourceSlotContent)) (.quantity (Utilities|Array|Get(acopy) (Variables|Default|GetItems) DestinationIndex))) 0 (CallFunction|GetItemMaxStack (.itemid (LocalVariables|GetL_SourceSlotContent)))) (.shielditemid (LocalVariables|GetL_SourceSlotContent))))))
    (CallFunction|MCUpdate)
    (CallFunction|MCUpdate SourceInventory)))

(fn IsEquipment
  (return (Utilities|ClassIsChildOf (Utilities|GetClass self) "/Game/Blueprints/Inventory/BP_PlayerEquipmentComponent.BP_PlayerEquipmentComponent_C")))

(fn QuickTransferwithOpenedStorage
  (params (SourceIndex :type Integer))
  (bind _returnvalue (Components|GetOwner))
  (bind _asbp_player_character (Utilities|Casting|CastToBP_PlayerCharacter _returnvalue)
    (:then
      (Utilities|IsValid (Variables|/Game/Blueprints/Player/BP_PlayerCharacter.BP_PlayerCharacter_C|GetOpenedStorage _asbp_player_character)
        (:Is%20Valid
          (LocalVariables|SetDestinationInventory (Variables|/Game/Blueprints/Placeable/Storages/BP_Storage.BP_Storage_C|GetBP_InventoryComponent (Variables|/Game/Blueprints/Player/BP_PlayerCharacter.BP_PlayerCharacter_C|GetOpenedStorage _asbp_player_character))))))
    (:CastFailed
      (Utilities|Casting|CastToBP_Storage _returnvalue)
      (LocalVariables|SetDestinationInventory (Variables|/Game/Blueprints/Player/BP_PlayerCharacter.BP_PlayerCharacter_C|GetBP_InventoryComponent (.AsBP%20Player%20Character (Utilities|Casting|CastToBP_PlayerCharacter (Pawn|GetControlledPawn (Game|GetPlayerController 0))))))))
  (bind _output (CallFunction|GetSlotItemStructbyIndex SourceIndex))
  (bind (_success _quantityremaining) (CallFunction|AddItem (LocalVariables|GetDestinationInventory) _output))
  (if _success
    (CallFunction|SubtractfromStack SourceIndex (- (.Quantity (Utilities|Struct|BreakS_SlotItem _output)) _quantityremaining))
    (CallFunction|MCUpdate)
    (CallFunction|MCUpdate (LocalVariables|GetDestinationInventory))))

(fn IsSlotHasItem
  (params (SlotIndex :type Integer))
  (bind _output (CallFunction|GetSlotItemStructbyIndex SlotIndex))
  (return (> (.quantity _output) 0)))

(fn PutbyIndex
  (params (Index :type Integer) (S_SlotItem :type S%20Slot%20Item%20Structure) (IsForce :type Boolean))
  (if IsForce
    (Utilities|Array|SetArrayElem (Variables|Default|GetItems) Index S_SlotItem :!label _label)
    (CallFunction|MCUpdate)
    (else
      (bind _output (CallFunction|GetSlotItemStructbyIndex Index))
      (if (not (> (.quantity _output) 0))
        (goto _label)))))