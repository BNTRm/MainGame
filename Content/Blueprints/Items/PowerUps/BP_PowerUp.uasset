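; Base power-up pickup actor that spins its static mesh every tick.
; It becomes pickupable after a short retriggerable delay on BeginPlay, so it cannot be grabbed the moment it spawns.
; PickUp checks that flag, calls the empty OnPickUp hook for child Blueprints to fill in, then destroys the actor.
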(event Custom|MakeTempNonPickupable
  (params (Secs :type Float%20%28double-precision%29))
  (Utilities|FlowControl|RetriggerableDelay Secs)
  (Variables|Default|SetIsPickupable true))

(event EventBeginPlay
  (CallFunction|MakeTempNonPickupable 0.2))

(event Collision|EventActorBeginOverlap
  (params (OtherActor :type Actor%20Object%20Reference)))

(event EventTick
  (params (DeltaSeconds :type Float%20%28single-precision%29))
  (Transformation|AddWorldRotation (Variables|Default|GetStaticMesh) "0,1.000000, 0" false false))

(fn ConstructionScript)

(fn PickUp
  (params (Pickuper :type Character%20Object%20Reference))
  (if (Variables|Default|GetIsPickupable)
    (CallFunction|OnPickUp Pickuper)
    (Actor|DestroyActor)))

(fn OnPickUp
  (params (Pickuper :type Character%20Object%20Reference)))