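; Placeable world object that occupies grid blocks and drops itself as an item when destroyed.
; Construction reads ExtraSize from DT_Items_Placeable by ItemId, then records BlockedLocations using the game mode's PlaceableObjectsManager, covering either one location or a box area.
; GetShiftVector returns the size's remainder against the block size, and LookAt returns an empty message and item.
; On destruction, DroppedItemsManager spawns one matching item, briefly non-pickable.
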(event EventDestroyed
  (bind _droppeditem (Default|SpawnDroppedItem (Variables|/Game/Blueprints/BP_GameMode.BP_GameMode_C|GetDroppedItemsManager (.AsBP%20Game%20Mode (Utilities|Casting|CastToBP_GameMode (Game|GetGameMode)))) (Transformation|GetWorldLocation (Variables|Default|GetDefaultSceneRoot)) (Variables|Default|GetItemId) 1 "0, 0, 0"))
  (Default|MakeTempNonPickapable _droppeditem 0.1))

(fn ConstructionScript
  (bind _itemid (Variables|Default|GetItemId))
  (Variables|Default|SetPlaceablesManager (Variables|/Game/Blueprints/BP_GameMode.BP_GameMode_C|GetPlaceableObjectsManager (.AsBP%20Game%20Mode (Utilities|Casting|CastToBP_GameMode (Game|GetGameMode)))))
  (bind _returnvalue (Utilities|GetDataTableRow "/Game/Data/Items/DT_Items_Placeable.DT_Items_Placeable" _itemid)
    (:then
      (Variables|Default|SetExtraSize (.extrasize _returnvalue))
      (if (!= _itemid "")
        (CallFunction|BlockLocations)))))

(fn BlockLocations
  (LocalVariables|SetL_Location (Transformation|GetWorldLocation (Variables|Default|GetStaticMesh)))
  (if (Utilities|Operators|NotEqual(!=) :A (Variables|Default|GetExtraSize) :ErrorTolerance 0.001)
    (for _array_element (Class|PlaceablesManager|FindLocationsinBoxArea (Variables|Default|GetPlaceablesManager) (LocalVariables|GetL_Location) (Variables|Default|GetExtraSize))
      (Utilities|Array|Add (Variables|Default|GetBlockedLocations) _array_element))
    (else
      (Utilities|Array|Add (Variables|Default|GetBlockedLocations) (LocalVariables|GetL_Location)))))

(fn GetShiftVector
  (bind _placeablesmanager (Variables|Default|GetPlaceablesManager))
  (bind _extrasize (Variables|Default|GetExtraSize))
  (bind _blocksize (Variables|/Script/MainGame.PlaceablesManager|GetBlockSize _placeablesmanager))
  (bind _returnvalue (Math|Conversions|ToFloat(Integer) _blocksize))
  (return (Math|Vector|MakeVector (Math|Float|%(Float) (.x _extrasize) _returnvalue) (Math|Float|%(Float) (.y _extrasize) _returnvalue) (Math|Float|%(Float) (.z _extrasize) _returnvalue))))

(fn Lookat
  (params (Observer :type BP%20Player%20Character%20Object%20Reference))
  (return "" "None"))