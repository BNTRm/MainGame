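; BP_PlacementPreview is the preview actor that shows whether a placeable item fits at its current spot.
; SetPreviewMesh swaps the mesh and reads the item's ExtraSize from DT_Items_Placeable.
; IsValid box-checks a slightly shrunk block-plus-ExtraSize volume for other placeables, players or creatures, and UpdateIsValid applies the valid or invalid material accordingly.
; An intentionally empty Destroyed event suppresses the parent's logic.
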(event EventDestroyed
  ;[1 1 1] Оставить, даже если пустой, чтобы не вызывался родительский
)

(fn ConstructionScript
  (|CallParentFunction))

(fn UpdateIsValid
  (bind _staticmesh (Variables|Default|GetStaticMesh))
  (if (CallFunction|IsValid)
    (Rendering|Material|SetMaterial _staticmesh 0 (Variables|Default|GetValidMaterial))
    (else
      (Rendering|Material|SetMaterial _staticmesh 0 (Variables|Default|GetInvalidMaterial)))))

(fn IsValid
  (bind _returnvalue (Class|KismetSystemLibrary|MakeLiteralInteger 2))
  (bind _returnvalue_2 (Class|KismetSystemLibrary|MakeLiteralInteger -2))
  (bind _array (Utilities|Array|MakeArray "ObjectTypeQuery3"))
  (bind _placeablesmanager (Variables|Default|GetPlaceablesManager))
  (bind _extrasize (Variables|Default|GetExtraSize))
  (bind _staticmesh (Variables|Default|GetStaticMesh))
  (bind _returnvalue_3 (Transformation|GetWorldLocation _staticmesh))
  (bind _blocksize (Variables|/Script/MainGame.PlaceablesManager|GetBlockSize _placeablesmanager))
  (bind _returnvalue_4 (Math|Conversions|ToVector(Float) _blocksize))
  (bind _returnvalue_5 (+ _returnvalue_4 _extrasize _returnvalue_2))
  (bind _returnvalue_6 (/ _returnvalue_5 _returnvalue))
  (bind _outactors (Collision|BoxOverlapActors _returnvalue_3 _returnvalue_6 (Utilities|Array|MakeArray "ObjectTypeQuery1") "/Game/Blueprints/Placeable/BP_Placeable.BP_Placeable_C" (Utilities|Array|MakeArray self) :!class /Script/Engine.KismetSystemLibrary))
  (bind _outactors_2 (Collision|BoxOverlapActors _returnvalue_3 _returnvalue_6 _array "/Game/Blueprints/Player/BP_PlayerCharacter.BP_PlayerCharacter_C" :!class /Script/Engine.KismetSystemLibrary))
  (bind _outactors_3 (Collision|BoxOverlapActors _returnvalue_3 _returnvalue_6 _array "/Game/Blueprints/Creatures/BP_Creature.BP_Creature_C" :!class /Script/Engine.KismetSystemLibrary))
  (return (Math|Boolean|ANDBoolean (== (Utilities|Array|Length _outactors) 0) (== (Utilities|Array|Length _outactors_2) 0) (== (Utilities|Array|Length _outactors_3) 0))))

(fn SetPreviewMesh
  (params (NewMesh :type Static%20Mesh%20Object%20Reference) (ItemId :type Name))
  (Components|StaticMesh|SetStaticMesh (Variables|Default|GetStaticMesh) NewMesh)
  (bind _returnvalue (Utilities|GetDataTableRow "/Game/Data/Items/DT_Items_Placeable.DT_Items_Placeable" ItemId)
    (:then
      (Variables|Default|SetExtraSize (.extrasize _returnvalue)))))