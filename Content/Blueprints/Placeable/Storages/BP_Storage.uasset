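; BP_Storage is a placeable storage container that holds items in an inventory component.
; Looking at it shows an "Open" prompt with the name looked up from the items data table.
; Interacting opens the storage menu on the first player's HUD, bound to that inventory.
; When destroyed, it spawns each stored item at its location through the game mode's dropped items manager, briefly blocking pickup.
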(event EventBeginPlay
  (|CallParentFunction) ; This node is disabled and will not be called.\nDrag off pins to build functionality.
)

(event Collision|EventActorBeginOverlap
  (params (OtherActor :type Actor%20Object%20Reference))
  (|CallParentFunction OtherActor) ; This node is disabled and will not be called.\nDrag off pins to build functionality.
)

(event EventTick
  (params (DeltaSeconds :type Float%20%28single-precision%29))
  (|CallParentFunction DeltaSeconds))

(event EventDestroyed
  (for _array_element (Variables|/Game/Blueprints/Inventory/BP_InventoryComponent.BP_InventoryComponent_C|GetItems (Variables|Default|GetBP_InventoryComponent))
    (bind _droppeditem (Default|SpawnDroppedItem (Variables|/Game/Blueprints/BP_GameMode.BP_GameMode_C|GetDroppedItemsManager (.AsBP%20Game%20Mode (Utilities|Casting|CastToBP_GameMode (Game|GetGameMode)))) (Transformation|GetWorldLocation (Variables|Default|GetDefaultSceneRoot)) (.ItemId (Utilities|Struct|BreakS_SlotItem _array_element)) (.Quantity (Utilities|Struct|BreakS_SlotItem _array_element)) "0, 0, 0"))
    (Default|MakeTempNonPickapable _droppeditem 0.1))
  (|CallParentFunction))

(event EventInteractwith
  (params (Interactor :type Character%20Object%20Reference))
  (bind _asbp_player_controller (Utilities|Casting|CastToBP_PlayerController (Game|GetPlayerController 0)))
  (Default|ToggleStorageMenu (Variables|/Game/Blueprints/Player/BP_PlayerController.BP_PlayerController_C|GetPlayerHudWidget _asbp_player_controller) true (Variables|Default|GetBP_InventoryComponent)))

(fn ConstructionScript
  (|CallParentFunction))

(fn Lookat
  (params (Observer :type BP%20Player%20Character%20Object%20Reference))
  (bind _returnvalue (Utilities|GetDataTableRow "/Game/MAIN_GAME/Data/Items/DT_Items.DT_Items" (Variables|Default|GetItemId))
    (:then
      (return (Utilities|Text|FormatText "Open \"{name}\"" (.Name (Utilities|Struct|BreakS_Item _returnvalue))) "None"))))