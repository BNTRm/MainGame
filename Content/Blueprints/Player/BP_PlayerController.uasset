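; Player controller that creates the local player's HUD and drives inventory and hotbar input, wrapping the selected slot and refreshing grids.
; In-menu key handlers close menus, drop items and track Shift.
; Right-click works through the drag-drop component to drop one, split stacks, pull shields or attach a dragged shield to an eligible weapon via DataTable lookups, or drop items on the drop button.
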(event EventBeginPlay
  (|DisplayPlayerHud))

(event Input|ActionEvents|InputActionInventory
  (params (Key :type Key%20Structure :default "None"))
  (:Pressed
    (Default|ToggleInventoryMenu (Variables|Default|GetPlayerHudWidget) true)))

(event Input|ActionEvents|InputActionNextHotbarSlot
  (params (Key :type Key%20Structure :default "None"))
  (bind _playerhudwidget (Variables|Default|GetPlayerHudWidget))
  (:Pressed
    (bind _result (Math|Integer|IncrementInt (Variables|Default|GetSelectedSlotIndex))
      (:%20%20
        (if (> _result 9)
          (Variables|Default|SetSelectedSlotIndex 0)
          (else
            (Variables|Default|SetSelectedSlotIndex _result)))
        (Default|UpdateGrid (Variables|/Game/Widgets/Inventory/WB_Hotbar.WB_Hotbar_C|GetWB_InventoryGrid (Variables|/Game/Widgets/PlayerHUD/WB_PlayerHud.WB_PlayerHud_C|GetWB_Hotbar _playerhudwidget)))
        (Default|UpdateGrid (Variables|/Game/Widgets/Inventory/WB_PlayerInventory.WB_PlayerInventory_C|GetWB_InventoryGrid (Variables|/Game/Widgets/PlayerHUD/WB_PlayerHud.WB_PlayerHud_C|GetWB_PlayerInventory _playerhudwidget)))
        (Default|UpdateGrid (Variables|/Game/Widgets/Inventory/WB_StorageInventory.WB_StorageInventory_C|GetWB_InventoryGrid (Variables|/Game/Widgets/PlayerHUD/WB_PlayerHud.WB_PlayerHud_C|GetWB_StorageInventory _playerhudwidget)))
        (Default|CallOnSelectedSlotIndexChanged)))))

(event Input|ActionEvents|InputActionPreviousHotbarSlot
  (params (Key :type Key%20Structure :default "None"))
  (bind _playerhudwidget (Variables|Default|GetPlayerHudWidget))
  (:Pressed
    (bind _result (Math|Integer|DecrementInt (Variables|Default|GetSelectedSlotIndex))
      (:%20%20
        (if (< _result 0)
          (Variables|Default|SetSelectedSlotIndex 9)
          (else
            (Variables|Default|SetSelectedSlotIndex _result)))
        (Default|UpdateGrid (Variables|/Game/Widgets/Inventory/WB_Hotbar.WB_Hotbar_C|GetWB_InventoryGrid (Variables|/Game/Widgets/PlayerHUD/WB_PlayerHud.WB_PlayerHud_C|GetWB_Hotbar _playerhudwidget)))
        (Default|UpdateGrid (Variables|/Game/Widgets/Inventory/WB_PlayerInventory.WB_PlayerInventory_C|GetWB_InventoryGrid (Variables|/Game/Widgets/PlayerHUD/WB_PlayerHud.WB_PlayerHud_C|GetWB_PlayerInventory _playerhudwidget)))
        (Default|UpdateGrid (Variables|/Game/Widgets/Inventory/WB_StorageInventory.WB_StorageInventory_C|GetWB_InventoryGrid (Variables|/Game/Widgets/PlayerHUD/WB_PlayerHud.WB_PlayerHud_C|GetWB_StorageInventory _playerhudwidget)))
        (Default|CallOnSelectedSlotIndexChanged)))))

(fn ConstructionScript)

(fn OnKeyDowninMenu
  (params (S_KeyEvent :type Key%20Event%20Structure))
  (bind _returnvalue (Class|InputSettings|GetInputSettings))
  (LocalVariables|SetL_Key (Class|KismetInputLibrary|GetKey S_KeyEvent))
  (if (== (LocalVariables|GetL_Key) (.key (Utilities|Array|Get(acopy) (Class|InputSettings|GetActionMappingbyName _returnvalue "Interact"))))
    (Default|CloseMenus (Variables|Default|GetPlayerHudWidget) :!label _label)
    (return (Class|WidgetBlueprintLibrary|Handled))
    (elif (== (LocalVariables|GetL_Key) (.key (Utilities|Array|Get(acopy) (Class|InputSettings|GetActionMappingbyName _returnvalue "Inventory"))))
      (goto _label)
      (elif (== (LocalVariables|GetL_Key) (.key (Utilities|Array|Get(acopy) (Class|InputSettings|GetActionMappingbyName _returnvalue "DropItem"))))
        (Default|DropItemfromMenu (.AsBP%20Player%20Character (Utilities|Casting|CastToBP_PlayerCharacter (Pawn|GetControlledPawn))))
        (return (Class|WidgetBlueprintLibrary|Handled))
        (elif (== (LocalVariables|GetL_Key) "LeftShift")
          (Variables|Default|SetIsShiftHolded true)
          (else
            (return (Class|WidgetBlueprintLibrary|Unhandled))))))))

(fn OnMouseButtonDowninMenu
  (params (S_PointerEvent :type Pointer%20Event%20Structure))
  (bind _bp_dragdropcomponent (Variables|Default|GetBP_DragDropComponent))
  (bind _output (Default|GetDraggableSlotItem _bp_dragdropcomponent))
  (if (Class|KismetInputLibrary|PointerEventIsMouseButtonDown S_PointerEvent "RightMouseButton")
    (Utilities|IsValid (Variables|/Game/Widgets/PlayerHUD/WB_PlayerHud.WB_PlayerHud_C|GetMouseHoveredSlot (Variables|Default|GetPlayerHudWidget))
      (:Is%20Valid
        (Utilities|GetDataTableRow "/Game/Data/Items/DT_Items_Shields.DT_Items_Shields" (.itemid _output)
          (:then
            (CallFunction|RMBPutShield (.itemid _output)))
          (:RowNotFound
            (CallFunction|RMBSplitSlot)))
        (return (Class|WidgetBlueprintLibrary|Handled)))
      (:Is%20Not%20Valid
        (if (Variables|/Game/Widgets/Inventory/WB_Drop.WB_Drop_C|GetIsButtonHovered (Variables|/Game/Widgets/PlayerHUD/WB_PlayerHud.WB_PlayerHud_C|GetWB_Drop (Variables|Default|GetPlayerHudWidget)))
          (Default|DropDraggableItem (Variables|Default|GetBP_DragDropComponent) 1))))
    (else
      (return (Class|WidgetBlueprintLibrary|Unhandled)))))

(fn OnKeyUpinMenu
  (params (S_KeyEvent :type Key%20Event%20Structure))
  (if (== (Class|KismetInputLibrary|GetKey S_KeyEvent) "LeftShift")
    (Variables|Default|SetIsShiftHolded false)
    (return (Class|WidgetBlueprintLibrary|Handled))
    (else
      (return (Class|WidgetBlueprintLibrary|Unhandled)))))

(fn RMBSplitSlot
  (bind _bp_dragdropcomponent (Variables|Default|GetBP_DragDropComponent))
  (bind _playerhudwidget (Variables|Default|GetPlayerHudWidget))
  (bind _playerhudwidget_2 (Variables|Default|GetPlayerHudWidget))
  (bind _playerhudwidget_3 (Variables|Default|GetPlayerHudWidget))
  (bind _mousehoveredslot (Variables|/Game/Widgets/PlayerHUD/WB_PlayerHud.WB_PlayerHud_C|GetMouseHoveredSlot _playerhudwidget))
  (bind _mousehoveredslot_2 (Variables|/Game/Widgets/PlayerHUD/WB_PlayerHud.WB_PlayerHud_C|GetMouseHoveredSlot _playerhudwidget_2))
  (bind _mousehoveredslot_3 (Variables|/Game/Widgets/PlayerHUD/WB_PlayerHud.WB_PlayerHud_C|GetMouseHoveredSlot _playerhudwidget_3))
  (bind _slotitemstruct (Variables|/Game/Widgets/Inventory/WB_InventorySlot.WB_InventorySlot_C|GetSlotItemStruct _mousehoveredslot_3))
  (bind _content_index (Variables|/Game/Widgets/Inventory/WB_InventorySlot.WB_InventorySlot_C|GetContent%20Index _mousehoveredslot_2))
  (bind _inventorycomponent (Variables|/Game/Widgets/Inventory/WB_InventorySlot.WB_InventorySlot_C|GetInventoryComponent _mousehoveredslot_2))
  (if (Default|IsDragging (Variables|Default|GetBP_DragDropComponent))
    (Default|DropOne (Variables|Default|GetBP_DragDropComponent) (Variables|/Game/Widgets/PlayerHUD/WB_PlayerHud.WB_PlayerHud_C|GetMouseHoveredSlot (Variables|Default|GetPlayerHudWidget)))
    (elif (!= (.quantity _slotitemstruct) 0)
      (if (== (.shielditemid _slotitemstruct) "")
        (if (> (.quantity _slotitemstruct) 1)
          (Default|StartDrag _bp_dragdropcomponent _inventorycomponent _content_index (Math|Float|Round (/ (Math|Conversions|ToFloat(Integer) (.quantity _slotitemstruct)) 2.0)))
          (else
            (Default|StartDrag _bp_dragdropcomponent _inventorycomponent _content_index)))
        (else
          (Default|PullShield (Variables|Default|GetBP_DragDropComponent) (Variables|/Game/Widgets/Inventory/WB_InventorySlot.WB_InventorySlot_C|GetInventoryComponent _mousehoveredslot) (Variables|/Game/Widgets/Inventory/WB_InventorySlot.WB_InventorySlot_C|GetContent%20Index _mousehoveredslot)))))))

(fn RMBPutShield
  (params (ShieldItemId :type Name))
  (bind _playerhudwidget (Variables|Default|GetPlayerHudWidget))
  (bind _playerhudwidget_2 (Variables|Default|GetPlayerHudWidget))
  (bind _mousehoveredslot (Variables|/Game/Widgets/PlayerHUD/WB_PlayerHud.WB_PlayerHud_C|GetMouseHoveredSlot _playerhudwidget))
  (bind _mousehoveredslot_2 (Variables|/Game/Widgets/PlayerHUD/WB_PlayerHud.WB_PlayerHud_C|GetMouseHoveredSlot _playerhudwidget_2))
  (bind _slotitemstruct (Variables|/Game/Widgets/Inventory/WB_InventorySlot.WB_InventorySlot_C|GetSlotItemStruct _mousehoveredslot_2))
  (bind _slotitemstruct_2 (Variables|/Game/Widgets/Inventory/WB_InventorySlot.WB_InventorySlot_C|GetSlotItemStruct _mousehoveredslot))
  (bind _returnvalue (Utilities|GetDataTableRow "/Game/Data/Items/DT_Items_Weapons.DT_Items_Weapons" (.itemid _slotitemstruct))
    (:then
      (if (and (Utilities|Enum|Equal(Enum) (.weapontype _returnvalue) "NewEnumerator0") (== (.shielditemid _slotitemstruct) ""))
        (Default|PutbyIndex (Variables|/Game/Widgets/Inventory/WB_InventorySlot.WB_InventorySlot_C|GetInventoryComponent _mousehoveredslot) (Variables|/Game/Widgets/Inventory/WB_InventorySlot.WB_InventorySlot_C|GetContent%20Index _mousehoveredslot) (Utilities|Struct|MakeS_SlotItem (.itemid _slotitemstruct_2) (.quantity _slotitemstruct_2) ShieldItemId) true)
        (Default|ClearDragSlot (Variables|Default|GetBP_DragDropComponent))))))