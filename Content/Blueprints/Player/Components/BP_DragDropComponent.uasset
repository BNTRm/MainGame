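; Player controller component that handles drag-and-drop of items between inventory slots and dropping them into the world.
; Slot 0 of the controller's DragDropInventoryComponent holds the dragged item, shown by the HUD drag preview.
; StartDrag moves a stack or quantity there; StopDrag and DropOne place it, checking slot types against DT_Items, with CancelDrag returning it.
; Attached shields can be pulled out, and spawn separately when dropped through the DroppedItemsManager.
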(event EventBeginPlay
  (bind _output_get (Variables|Default|SetPlayerController (.AsBP%20Player%20Controller (Utilities|Casting|CastToBP_PlayerController (Game|GetPlayerController 0)))))
  (Variables|Default|SetDragDropInventoryComponent (Variables|/Game/Blueprints/Player/BP_PlayerController.BP_PlayerController_C|GetDragDropInventoryComponent _output_get))
  (EventDispatchers|BindEventtoOnInventoryUpdated (Variables|/Game/Blueprints/Player/BP_PlayerController.BP_PlayerController_C|GetDragDropInventoryComponent _output_get) (EventDispatchers|CreateEvent :!event UpdateWidget)))

(fn StartDrag
  (params (SourceInventory :type BP%20Inventory%20Component%20Object%20Reference) (SourceIndex :type Integer) (Quantity :type Integer))
  (Variables|Default|SetDragSourceInventory SourceInventory)
  (bind _output_get (Variables|Default|SetDragSourceIndex SourceIndex))
  (if (== Quantity 0)
    (Default|TransferSlots (Variables|Default|GetDragDropInventoryComponent) (Variables|Default|GetDragSourceIndex) (Variables|Default|GetDragSourceInventory))
    (if (CallFunction|IsDragging) :!label _label
      (CallFunction|UpdateWidget))
    (else
      (bind _output (Default|GetSlotItemStructbyIndex SourceInventory _output_get))
      (bind _success (Default|AddItem (Variables|Default|GetDragDropInventoryComponent) (Utilities|Struct|MakeS_SlotItem (.itemid _output) Quantity (.shielditemid _output))))
      (if _success
        (Default|SubtractfromStack SourceInventory SourceIndex Quantity)
        (goto _label)))))

(fn StopDrag
  (params (DestinationInventory :type BP%20Inventory%20Component%20Object%20Reference) (DestinationIndex :type Integer) (DestinationSlotType :type EN_SlotType%20Enum :default "NewEnumerator0"))
  (bind _playercontroller (Variables|Default|GetPlayerController))
  (bind _bp_dragdropcomponent (Variables|/Game/Blueprints/Player/BP_PlayerController.BP_PlayerController_C|GetBP_DragDropComponent _playercontroller))
  (if (CallFunction|IsDragging _bp_dragdropcomponent)
    (Utilities|IsValid DestinationInventory
      (:Is%20Valid
        (bind _returnvalue (Utilities|GetDataTableRow "/Game/MAIN_GAME/Data/Items/DT_Items.DT_Items" (.itemid (CallFunction|GetDraggableSlotItem _bp_dragdropcomponent)))
          (:then
            (if (Default|IsEquipment DestinationInventory)
              (if (Utilities|Enum|Equal(Enum) DestinationSlotType (.SlotType (Utilities|Struct|BreakS_Item _returnvalue)))
                (Default|TransferSlots DestinationInventory 0 (Variables|Default|GetDragDropInventoryComponent) DestinationIndex :!label _label)
                (if (CallFunction|IsDragging (Variables|/Game/Blueprints/Player/BP_PlayerController.BP_PlayerController_C|GetBP_DragDropComponent (Variables|Default|GetPlayerController)))
                  (Default|Update (Variables|/Game/Widgets/PlayerHUD/WB_PlayerHud.WB_PlayerHud_C|GetWB_DragPreview (Variables|/Game/Blueprints/Player/BP_PlayerController.BP_PlayerController_C|GetPlayerHudWidget (Variables|Default|GetPlayerController))))
                  (else
                    (CallFunction|ClearDragSlot :!label _label_2))))
              (else
                (goto _label))))
          (:RowNotFound
            (Default|TransferSlots (Variables|Default|GetDragSourceInventory) 0 (Variables|Default|GetDragDropInventoryComponent) (Variables|Default|GetDragSourceIndex) :!label _label_3)
            (CallFunction|CancelDrag)
            (goto _label_2))))
      (:Is%20Not%20Valid
        (goto _label_3)))
    (else
      (goto _label_2))))

(fn DropDraggableItem
  (params (Amount :type Integer))
  (bind _output (CallFunction|GetDraggableSlotItem))
  (bind _output_2 (CallFunction|GetDraggableSlotItem))
  (bind _returnvalue (Game|GetGameMode))
  (bind _playercontroller (Variables|Default|GetPlayerController))
  (bind _returnvalue_2 (Pawn|GetControlledPawn _playercontroller))
  (bind _asbp_game_mode (Utilities|Casting|CastToBP_GameMode _returnvalue))
  (bind _asbp_player_character (Utilities|Casting|CastToBP_PlayerCharacter _returnvalue_2))
  (bind _droppeditemsmanager (Variables|/Game/Blueprints/BP_GameMode.BP_GameMode_C|GetDroppedItemsManager _asbp_game_mode))
  (bind _dropimpulsemultiplier (Variables|/Game/Blueprints/Player/BP_PlayerCharacter.BP_PlayerCharacter_C|GetDropImpulseMultiplier _asbp_player_character))
  (bind _capsulecomponent (Variables|/Script/Engine.Character|GetCapsuleComponent _asbp_player_character))
  (bind _returnvalue_3 (Math|Vector|GetForwardVector _capsulecomponent))
  (bind _returnvalue_4 (Transformation|GetWorldLocation _capsulecomponent))
  (bind _returnvalue_5 (* _returnvalue_3 _dropimpulsemultiplier))
  (if (== Amount 0)
    (LocalVariables|SetL_Amount (.quantity _output_2))
    (else
      (LocalVariables|SetL_Amount Amount)))
  (Default|SpawnDroppedItem _droppeditemsmanager _returnvalue_4 (.itemid _output_2) (LocalVariables|GetL_Amount) _returnvalue_5)
  (if (!= (.shielditemid _output) "")
    (Default|SpawnDroppedItem _droppeditemsmanager _returnvalue_4 (.shielditemid _output) 1 _returnvalue_5))
  (Default|SubtractfromStack (Variables|Default|GetDragDropInventoryComponent) 0 (LocalVariables|GetL_Amount)))

(fn IsDragging
  (bind _playercontroller (Variables|Default|GetPlayerController))
  (bind _bp_dragdropcomponent (Variables|/Game/Blueprints/Player/BP_PlayerController.BP_PlayerController_C|GetBP_DragDropComponent _playercontroller))
  (bind _output (CallFunction|GetDraggableSlotItem _bp_dragdropcomponent))
  (return (and (!= (.itemid _output) "") (> (.quantity _output) 0))))

(fn CancelDrag
  (if (Default|IsSlotHasItem (Variables|Default|GetDragSourceInventory) (Variables|Default|GetDragSourceIndex))
    (bind _output (Default|GetSlotItemStructbyIndex (Variables|Default|GetDragDropInventoryComponent)))
    (Default|AddItem (Variables|Default|GetDragSourceInventory) _output)
    (CallFunction|ClearDragSlot)
    (else
      (Default|TransferSlots (Variables|Default|GetDragSourceInventory) 0 (Variables|Default|GetDragDropInventoryComponent) (Variables|Default|GetDragSourceIndex)))))

(fn ClearDragSlot
  (Widget|SetVisibility (Variables|/Game/Widgets/PlayerHUD/WB_PlayerHud.WB_PlayerHud_C|GetWB_DragPreview (Variables|/Game/Blueprints/Player/BP_PlayerController.BP_PlayerController_C|GetPlayerHudWidget (Variables|Default|GetPlayerController))) "Hidden")
  (Utilities|Array|SetArrayElem (Variables|/Game/Blueprints/Inventory/BP_InventoryComponent.BP_InventoryComponent_C|GetItems (Variables|Default|GetDragDropInventoryComponent)) 0 (Utilities|Struct|MakeS_SlotItem "None" 0 "None")))

(fn DropOne
  (params (DestinationSlot :type WB%20Inventory%20Slot%20Object%20Reference))
  (bind _output (CallFunction|GetDraggableSlotItem))
  (bind _inventorycomponent (Variables|/Game/Widgets/Inventory/WB_InventorySlot.WB_InventorySlot_C|GetInventoryComponent DestinationSlot))
  (bind _type (Variables|/Game/Widgets/Inventory/WB_InventorySlot.WB_InventorySlot_C|GetType DestinationSlot))
  (bind _content_index (Variables|/Game/Widgets/Inventory/WB_InventorySlot.WB_InventorySlot_C|GetContent%20Index DestinationSlot))
  (if (CallFunction|IsDragging)
    (bind _output_2 (Default|GetSlotItemStructbyIndex (Variables|/Game/Widgets/Inventory/WB_InventorySlot.WB_InventorySlot_C|GetInventoryComponent DestinationSlot) (Variables|/Game/Widgets/Inventory/WB_InventorySlot.WB_InventorySlot_C|GetContent%20Index DestinationSlot)))
    (bind _returnvalue (Utilities|GetDataTableRow "/Game/MAIN_GAME/Data/Items/DT_Items.DT_Items" (.itemid (CallFunction|GetDraggableSlotItem)))
      (:then
        (if (or (Utilities|Enum|Equal(Enum) _type "NewEnumerator0") (Utilities|Enum|Equal(Enum) _type (.SlotType (Utilities|Struct|BreakS_Item _returnvalue))))
          (if (== (.ItemId (Utilities|Struct|BreakS_SlotItem _output_2)) (.itemid _output))
            (Default|AddtoStack _inventorycomponent _content_index 1)
            (Default|SubtractfromStack (Variables|Default|GetDragDropInventoryComponent) 0 1 :!label _label)
            (Default|MCUpdate (Variables|/Game/Widgets/Inventory/WB_InventorySlot.WB_InventorySlot_C|GetInventoryComponent DestinationSlot))
            (elif (== (.Quantity (Utilities|Struct|BreakS_SlotItem _output_2)) 0)
              (Default|PutbyIndex _inventorycomponent _content_index (Utilities|Struct|MakeS_SlotItem (.itemid _output) 1 (.shielditemid _output)) false)
              (goto _label))))))))

(fn GetDraggableSlotItem
  (return (Utilities|Array|Get(acopy) (Variables|/Game/Blueprints/Inventory/BP_InventoryComponent.BP_InventoryComponent_C|GetItems (Variables|Default|GetDragDropInventoryComponent)))))

(fn PullShield
  (params (SourceInventory :type BP%20Inventory%20Component%20Object%20Reference) (SourceIndex :type Integer))
  (bind _output (Default|GetSlotItemStructbyIndex SourceInventory SourceIndex))
  (Default|PutbyIndex (Variables|Default|GetDragDropInventoryComponent) 0 (Utilities|Struct|MakeS_SlotItem (.shielditemid _output) 1 "None") false)
  (Default|PutbyIndex SourceInventory SourceIndex (Utilities|Struct|MakeS_SlotItem (.itemid _output) (.quantity _output) "None") true))

(fn UpdateWidget
  (bind _playercontroller (Variables|Default|GetPlayerController))
  (bind _playerhudwidget (Variables|/Game/Blueprints/Player/BP_PlayerController.BP_PlayerController_C|GetPlayerHudWidget _playercontroller))
  (bind _wb_dragpreview (Variables|/Game/Widgets/PlayerHUD/WB_PlayerHud.WB_PlayerHud_C|GetWB_DragPreview _playerhudwidget))
  (Default|Update _wb_dragpreview)
  (Widget|SetVisibility _wb_dragpreview "Visible"))