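; Player component that plays action montages on the player character's mesh for placing, pickaxe hits, one-handed attacks and shield blocks.
; An action state selects the montage, and place and pickaxe repeat on completion while their fire input is held.
; One-handed attacks alternate right-to-left and left-to-right swings while fire is held.
; When a chain ends, it clears the current montage, which backs the is-playing check, and fires a completion callback.
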(event Custom|PlayMontageByAction
  (params (ActionState :type EN_ActionState%20Enum :default "NewEnumerator3"))
  (bind _player (Variables|Default|GetPlayer))
  (bind _isfireholding (Variables|/Game/Blueprints/Player/BP_PlayerCharacter.BP_PlayerCharacter_C|GetIsFireHolding _player))
  (switch Utilities|FlowControl|Switch|SwitchonEN_ActionState ActionState
    (:NewEnumerator0
      (bind _output_get (Variables|Default|SetCurrentMontage "/Game/Animations/Player/Actions/AM_Place.AM_Place"))
      (Animation|Montage|PlayMontage (Variables|/Script/Engine.Character|GetMesh (Variables|Default|GetPlayer)) _output_get :!label _label
        (:OnCompleted
          (if (Variables|/Game/Blueprints/Player/BP_PlayerCharacter.BP_PlayerCharacter_C|GetIsAltFireHolding (Variables|Default|GetPlayer))
            (goto _label)
            (else
              _)))))
    (:NewEnumerator5
      (bind _output_get_2 (Variables|Default|SetCurrentMontage "/Game/Animations/Player/Actions/AM_PickaxeHit.AM_PickaxeHit"))
      (Animation|Montage|PlayMontage (Variables|/Script/Engine.Character|GetMesh (Variables|Default|GetPlayer)) _output_get_2 :!label _label_2
        (:OnCompleted
          (if _isfireholding
            (goto _label_2)
            (else
              _)))))
    (:NewEnumerator6
      (bind _output_get_3 (Variables|Default|SetCurrentMontage "/Game/Animations/Player/Actions/AM_Attack_OneHanded_RtoL.AM_Attack_OneHanded_RtoL" :!label _label_3))
      (Animation|Montage|PlayMontage (Variables|/Script/Engine.Character|GetMesh (Variables|Default|GetPlayer)) _output_get_3
        (:OnCompleted
          (if _isfireholding
            (bind _output_get_4 (Variables|Default|SetCurrentMontage "/Game/Animations/Player/Actions/AM_Attack_OneHanded_LtoR.AM_Attack_OneHanded_LtoR"))
            (Animation|Montage|PlayMontage (Variables|/Script/Engine.Character|GetMesh (Variables|Default|GetPlayer)) _output_get_4
              (:OnCompleted
                (if _isfireholding
                  (goto _label_3)
                  (else
                    _))))))))
    (:NewEnumerator7
      (bind _output_get_5 (Variables|Default|SetCurrentMontage "/Game/Animations/Player/Actions/AM_ShieldBlock.AM_ShieldBlock"))
      (Animation|Montage|PlayMontage (Variables|/Script/Engine.Character|GetMesh (Variables|Default|GetPlayer)) _output_get_5
        (:OnCompleted
          _))))
  (Variables|Default|SetCurrentMontage 0)
  (Default|CallOnMontageCompleted))

(event EventBeginPlay
  (Variables|Default|SetPlayer (.AsBP%20Player%20Character (Utilities|Casting|CastToBP_PlayerCharacter (Components|GetOwner)))))

(fn IsMontagePlaying
  (return (!= (Variables|Default|GetCurrentMontage) 0)))