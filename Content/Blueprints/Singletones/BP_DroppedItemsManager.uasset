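; BP_DroppedItemsManager is a manager that spawns dropped items and power-ups into the world through SpawnDroppedItem.
; It looks up the ItemId in DT_Items, spawns that row's dropped Blueprint, stacks it for quantities above one and returns it.
; A second lookup in DT_PowerUps spawns power-up actors inside a Quantity-based loop that contains a return.
; Spawns get a physics impulse: a random upward scatter when none is supplied, otherwise the given one with jitter.
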(event EventBeginPlay)

(event Collision|EventActorBeginOverlap
  (params (OtherActor :type Actor%20Object%20Reference)))

(event EventTick
  (params (DeltaSeconds :type Float%20%28single-precision%29)))

(fn ConstructionScript)

(fn SpawnDroppedItem
  (params (Location :type Vector) (ItemId :type Name) (Quantity :type Integer) (Impulse :type Vector))
  (bind _returnvalue (Math|Random|RandomFloatinRange -1e+01 1e+01))
  (bind _returnvalue_2 (Math|Float|MakeLiteralFloat 2e+02))
  (bind _returnvalue_3 (Class|KismetMathLibrary|EqualExactlyVectorVector Impulse "0, 0, 0"))
  (bind _returnvalue_4 (* _returnvalue_2 -1.0))
  (bind _returnvalue_5 (+ Impulse _returnvalue))
  (bind _returnvalue_6 (Math|Random|RandomFloatinRange _returnvalue_4 _returnvalue_2))
  (bind _returnvalue_7 (Math|Random|RandomFloatinRange _returnvalue_4 _returnvalue_2))
  (bind _returnvalue_8 (Math|Vector|MakeVector _returnvalue_6 _returnvalue_7 _returnvalue_2))
  (bind _returnvalue_9 (select _returnvalue_3 _returnvalue_8 _returnvalue_5))
  (Utilities|FlowControl|Sequence
    (:then_0
      (bind _returnvalue_10 (Utilities|GetDataTableRow "/Game/Data/Items/DT_Items.DT_Items" ItemId)
        (:then
          (bind _returnvalue_11 (Game|SpawnActorfromClass (.Dropped_BPClass (Utilities|Struct|BreakS_Item _returnvalue_10)) (Math|Transform|MakeTransform Location "0, 0, 0" "1.000000,1.000000,1.000000") "Undefined" "SelectDefaultAtRuntime" 0 0))
          (if (> Quantity 1)
            (Default|ToStack _returnvalue_11 Quantity))
          (Physics|AddImpulse (Variables|/Game/Blueprints/Items/BP_Item_Dropped.BP_Item_Dropped_C|GetPhysicsCollision _returnvalue_11) _returnvalue_9 "None" false)
          (return _returnvalue_11))))
    (:then_1
      (bind _returnvalue_12 (Utilities|GetDataTableRow "/Game/Data/Items/DT_PowerUps.DT_PowerUps" ItemId)
        (:then
          (bind _result (Math|Integer|DecrementInt Quantity)
            (:%20%20
              (Utilities|FlowControl|ForLoopwithBreak 0 _result
                (:LoopBody
                  (bind _returnvalue_13 (Game|SpawnActorfromClass (Utilities|Struct|BreakS_PowerUp _returnvalue_12) (Math|Transform|MakeTransform Location "0, 0, 0" "1.000000,1.000000,1.000000") "Undefined" "SelectDefaultAtRuntime" 0 0))
                  (Physics|AddImpulse (Variables|/Game/Blueprints/Items/PowerUps/BP_PowerUp.BP_PowerUp_C|GetStaticMesh _returnvalue_13) _returnvalue_9 "None" false))
                (:Completed
                  (return 0))))))))))