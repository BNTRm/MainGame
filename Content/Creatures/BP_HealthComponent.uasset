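; Health component for creatures that tracks Health against MaxHealth.
; TakeDamage subtracts damage and floors Health at zero, while Heal adds a value and caps it at MaxHealth.
; It only changes the stored value, with no death handling or notifications, and its BeginPlay and Tick events are unused.
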(event EventBeginPlay)

(event EventTick
  (params (DeltaSeconds :type Float%20%28single-precision%29)))

(fn TakeDamage
  (params (Damage :type Integer))
  (if (< (- (Variables|Default|GetHealth) Damage) 0)
    (Variables|Default|SetHealth 0)
    (else
      (Variables|Default|SetHealth (- (Variables|Default|GetHealth) Damage)))))

(fn Heal
  (params (Value :type Integer))
  (if (> (+ Value (Variables|Default|GetHealth)) (Variables|Default|GetMaxHealth))
    (Variables|Default|SetHealth (Variables|Default|GetMaxHealth))
    (else
      (Variables|Default|SetHealth (+ Value (Variables|Default|GetHealth))))))