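; BP_Storage_Box is a storage box block that opens a storage menu when interacted with.
; Interactwith casts player controller 0 to BP_PlayerController and passes the box's BPInventoryComponent to DisplayStorageMenu on its PlayerHudWidget.
; LookAt returns an empty message and no item, and the construction script only calls its parent.
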(event EventBeginPlay
  (|CallParentFunction) ; This node is disabled and will not be called.\nDrag off pins to build functionality.
)

(event Collision|EventActorBeginOverlap
  (params (OtherActor :type Actor%20Object%20Reference))
  (|CallParentFunction OtherActor) ; This node is disabled and will not be called.\nDrag off pins to build functionality.
)

(event EventTick
  (params (DeltaSeconds :type Float%20%28single-precision%29))
  (|CallParentFunction DeltaSeconds) ; This node is disabled and will not be called.\nDrag off pins to build functionality.
)

(event EventInteractwith
  (params (Interactor :type Character%20Object%20Reference))
  (bind _asbp_player_controller (Utilities|Casting|CastToBP_PlayerController (Game|GetPlayerController 0)))
  (Default|DisplayStorageMenu (Variables|/Game/MAIN_GAME/Player/Blueprints/BP_PlayerController.BP_PlayerController_C|GetPlayerHudWidget _asbp_player_controller) (Variables|Default|GetBP_InventoryComponent)))

(fn ConstructionScript
  (|CallParentFunction))

(fn Lookat
  (params (Observer :type Voxman%20Character%20Object%20Reference))
  (return "" "None"))