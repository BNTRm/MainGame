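; Game mode that handles placing and breaking grid-aligned objects in a voxel-style world.
; Player placement rounds world coordinates to block coordinates, resolving half-block ties toward the player's active camera, then spawns the actor at the converted position.
; The rounding mixes BlockSize with a hard-coded 64-unit block.
; Breaking destroys the actor immediately; a comment marks hit points and item drops as planned.
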(event EventBeginPlay)

(event EventTick
  (params (DeltaSeconds :type Float%20%28single-precision%29)))

(fn ConstructionScript)

(fn SpawnActorbyGameCoords
  (params (Class :type Actor%20Class%20Reference) (WorldCoordX :type Integer) (WorldCoordY :type Integer) (WorldCoordZ :type Integer) (Instigator :type Pawn%20Object%20Reference))
  (bind _returnvalue (Game|SpawnActorfromClass Class (Math|Transform|MakeTransform (Math|Vector|MakeVector (Math|Conversions|ToFloat(Integer) (Class|MyGameMode|ConvertGametoWorldCoord WorldCoordX)) (Math|Conversions|ToFloat(Integer) (Class|MyGameMode|ConvertGametoWorldCoord WorldCoordY)) (Math|Conversions|ToFloat(Integer) (Class|MyGameMode|ConvertGametoWorldCoord WorldCoordZ))) "0, 0, 0" "1.000000,1.000000,1.000000") "AdjustIfPossibleButAlwaysSpawn" 0 Instigator))
  (return _returnvalue))

(fn WorldtoGameCoord
  (params (WorldCoord :type Float%20%28double-precision%29) (PositionCoord :type Float%20%28double-precision%29))
  (bind _returnvalue (Class|MyGameMode|Precision WorldCoord 3))
  (bind _returnvalue_2 (Math|Float|Round _returnvalue))
  (LocalVariables|SetRoundedWorldCoord _returnvalue_2)
  (LocalVariables|SetRoughGameCoord (/ _returnvalue_2 (Variables|Default|GetBlockSize)))
  (if (== (Math|Integer|%(Integer) (LocalVariables|GetRoundedWorldCoord) 64) 0)
    (return (LocalVariables|GetRoughGameCoord))
    (elif (== (Math|Integer|Absolute(Integer) (Math|Integer|%(Integer) (LocalVariables|GetRoundedWorldCoord) 64)) 32)
      (if (> PositionCoord WorldCoord)
        (return (+ (/ (+ (Math|Integer|%(Integer) (LocalVariables|GetRoundedWorldCoord) 64) 32) 64) (LocalVariables|GetRoughGameCoord)))
        (else
          (return (+ (/ (- (Math|Integer|%(Integer) (LocalVariables|GetRoundedWorldCoord) 64) 32) 64) (LocalVariables|GetRoughGameCoord)))))
      (elif (< (Math|Integer|Absolute(Integer) (Math|Integer|%(Integer) (LocalVariables|GetRoundedWorldCoord) 64)) 32)
        (return (LocalVariables|GetRoughGameCoord))
        (else
          (return (+ (/ (LocalVariables|GetRoundedWorldCoord) (Math|Integer|Absolute(Integer) (LocalVariables|GetRoundedWorldCoord))) (LocalVariables|GetRoughGameCoord))))))))

(fn PlaceObjectbyPlayer
  (params (Class :type Actor%20Class%20Reference) (WorldCoordX :type Float%20%28double-precision%29) (WorldCoordY :type Float%20%28double-precision%29) (WorldCoordZ :type Float%20%28double-precision%29) (Player :type Character%20Object%20Reference))
  (bind _asbp_player_character (Utilities|Casting|CastToBP_PlayerCharacter Player))
  (LocalVariables|SetVoxmanCharacter _asbp_player_character)
  (bind _resultcoord (CallFunction|WorldtoGameCoord WorldCoordX (.x (Transformation|GetWorldLocation (Default|GetActiveCamera (LocalVariables|GetVoxmanCharacter))))))
  (bind _resultcoord_2 (CallFunction|WorldtoGameCoord WorldCoordY (.y (Transformation|GetWorldLocation (Default|GetActiveCamera (LocalVariables|GetVoxmanCharacter))))))
  (bind _resultcoord_3 (CallFunction|WorldtoGameCoord WorldCoordZ (.z (Transformation|GetWorldLocation (Default|GetActiveCamera (LocalVariables|GetVoxmanCharacter))))))
  (bind _spawnedactor (CallFunction|SpawnActorbyGameCoords Class _resultcoord _resultcoord_2 _resultcoord_3))
  (return _spawnedactor))

(fn BreakObject
  (params (Actor :type Actor%20Object%20Reference))
  ;[1 0 0] Здесь будет отнимание ХП у объекта. По достижению 0 ХП объект уничтожается и выпадает (если может)
  (Actor|DestroyActor Actor))