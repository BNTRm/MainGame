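; Helper actor that spawns dropped items into the world as physics objects.
; SpawnDroppedItem looks up the item ID in DT_Items and spawns that row's dropped Blueprint class at the given location, stacking it when quantity exceeds one.
; It then applies an impulse to the item's physics collision, substituting a randomized sideways, upward toss when the supplied impulse is zero.
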(event EventBeginPlay)

(event Collision|EventActorBeginOverlap
  (params (OtherActor :type Actor%20Object%20Reference)))

(event EventTick
  (params (DeltaSeconds :type Float%20%28single-precision%29)))

(fn ConstructionScript)

(fn SpawnDroppedItem
  (params (Location :type Vector) (ItemId :type Name) (Quantity :type Integer) (Impulse :type Vector))
  (bind _returnvalue (Math|Float|MakeLiteralFloat 2e+02))
  (bind _returnvalue_2 (* _returnvalue -1.0))
  (bind _returnvalue_3 (Utilities|GetDataTableRow "/Game/MAIN_GAME/Data/Items/DT_Items.DT_Items" ItemId)
    (:then
      (bind _returnvalue_4 (Game|SpawnActorfromClass (.Dropped_BPClass (Utilities|Struct|BreakS_Item _returnvalue_3)) (Math|Transform|MakeTransform Location "0, 0, 0" "1.000000,1.000000,1.000000") "Undefined" 0 0))
      (if (> Quantity 1)
        (Default|ToStack _returnvalue_4 Quantity))
      (Physics|AddImpulse (Variables|/Game/MAIN_GAME/Blueprints/Items/BP_Item_Dropped.BP_Item_Dropped_C|GetPhysicsCollision _returnvalue_4) (select (Class|KismetMathLibrary|EqualExactlyVectorVector Impulse "0, 0, 0") (Math|Vector|MakeVector (Math|Random|RandomFloatinRange _returnvalue_2 _returnvalue) (Math|Random|RandomFloatinRange _returnvalue_2 _returnvalue) _returnvalue) Impulse) "None" false)
      (return _returnvalue_4))))