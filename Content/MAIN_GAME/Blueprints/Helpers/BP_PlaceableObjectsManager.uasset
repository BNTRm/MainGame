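; BP_PlaceableObjectsManager is a helper that spawns placeable objects, or previews of them, where the player aims.
; PlaceObjectByPlayer snaps the player character's crosshair impact point to a fixed 16-unit grid and spawns with zero rotation.
; It uses PreviewClass for previews and the Blueprint class from the held item's placeable struct otherwise.
; The spawned actor is returned with the player as instigator, adjusting for collision but always spawning.
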(event EventBeginPlay)

(event Collision|EventActorBeginOverlap
  (params (OtherActor :type Actor%20Object%20Reference)))

(event EventTick
  (params (DeltaSeconds :type Float%20%28single-precision%29)))

(fn ConstructionScript)

(fn PlaceObjectbyPlayer
  (params (Player :type Character%20Object%20Reference) (IsPreview :type Boolean))
  (bind _asbp_player_character (Utilities|Casting|CastToBP_PlayerCharacter Player)
    (:then
      (LocalVariables|SetPlayerCharacter _asbp_player_character)
      (bind _itemstruct (Default|GetHandsItemStructPlaceable (LocalVariables|GetPlayerCharacter)))
      (if IsPreview
        (bind _returnvalue (Game|SpawnActorfromClass (LocalVariables|GetPreviewClass) (Math|Transform|MakeTransform (Math|Vector|MakeVector (Math|Float|SnapToGrid(Float) (.X (Math|Vector|BreakVector (.impactpoint (Variables|/Game/MAIN_GAME/Blueprints/Player/BP_PlayerCharacter.BP_PlayerCharacter_C|GetCrosshairHitResult _asbp_player_character)))) 16.0) (Math|Float|SnapToGrid(Float) (.Y (Math|Vector|BreakVector (.impactpoint (Variables|/Game/MAIN_GAME/Blueprints/Player/BP_PlayerCharacter.BP_PlayerCharacter_C|GetCrosshairHitResult _asbp_player_character)))) 16.0) (Math|Float|SnapToGrid(Float) (.Z (Math|Vector|BreakVector (.impactpoint (Variables|/Game/MAIN_GAME/Blueprints/Player/BP_PlayerCharacter.BP_PlayerCharacter_C|GetCrosshairHitResult _asbp_player_character)))) 16.0))) "AdjustIfPossibleButAlwaysSpawn" 0 (LocalVariables|GetPlayerCharacter)))
        (return _returnvalue)
        (else
          (bind _returnvalue_2 (Game|SpawnActorfromClass (.placeable_bpclass _itemstruct) (Math|Transform|MakeTransform (Math|Vector|MakeVector (Math|Float|SnapToGrid(Float) (.X (Math|Vector|BreakVector (.impactpoint (Variables|/Game/MAIN_GAME/Blueprints/Player/BP_PlayerCharacter.BP_PlayerCharacter_C|GetCrosshairHitResult _asbp_player_character)))) 16.0) (Math|Float|SnapToGrid(Float) (.Y (Math|Vector|BreakVector (.impactpoint (Variables|/Game/MAIN_GAME/Blueprints/Player/BP_PlayerCharacter.BP_PlayerCharacter_C|GetCrosshairHitResult _asbp_player_character)))) 16.0) (Math|Float|SnapToGrid(Float) (.Z (Math|Vector|BreakVector (.impactpoint (Variables|/Game/MAIN_GAME/Blueprints/Player/BP_PlayerCharacter.BP_PlayerCharacter_C|GetCrosshairHitResult _asbp_player_character)))) 16.0))) "AdjustIfPossibleButAlwaysSpawn" 0 (LocalVariables|GetPlayerCharacter)))
          (return _returnvalue_2))))
    (:CastFailed
      (return 0))))