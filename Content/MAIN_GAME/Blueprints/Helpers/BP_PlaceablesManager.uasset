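; Placeables manager that spawns a player's held placeable, or a preview actor, at a grid-snapped point under the crosshair.
; PlaceObjectByPlayer takes the held item's placeable data from BP_PlayerCharacter and spawns PreviewClass or the item's Blueprint class.
; The location snaps the crosshair hit to BlockSize, shifted by half the ExtraSize remainder over a double block.
; Items with non-zero ExtraSize also move up to one block, using hit normals and trace direction signs.
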(fn ConstructionScript)

(fn PlaceObjectbyPlayer
  (params (Player :type Character%20Object%20Reference) (IsPreview :type Boolean))
  (bind _asbp_player_character (Utilities|Casting|CastToBP_PlayerCharacter Player)
    (:then
      (bind _output_get (LocalVariables|SetPlayerCharacter _asbp_player_character))
      (bind _itemstruct (Default|GetHandsItemStructPlaceable (LocalVariables|GetPlayerCharacter)))
      (if IsPreview
        (bind _returnvalue (Game|SpawnActorfromClass (LocalVariables|GetPreviewClass) (Math|Transform|MakeTransform (CallFunction|GetLoactionforPlacebyPlayer _output_get) "0, 0, 0" "1.000000,1.000000,1.000000") "AdjustIfPossibleButAlwaysSpawn" 0 (LocalVariables|GetPlayerCharacter)))
        (return _returnvalue)
        (else
          (bind _returnvalue_2 (Game|SpawnActorfromClass (.placeable_bpclass _itemstruct) (Math|Transform|MakeTransform (CallFunction|GetLoactionforPlacebyPlayer _output_get) "0, 0, 0" "1.000000,1.000000,1.000000") "AdjustIfPossibleButAlwaysSpawn" 0 (LocalVariables|GetPlayerCharacter)))
          (return _returnvalue_2))))
    (:CastFailed
      (return 0))))

(fn SnapLocationtoGrid
  (params (Location :type Vector) (Shift :type Vector))
  (return (+ (Class|KismetMathLibrary|VectorSnappedtoGrid (- Location Shift) (Math|Conversions|ToFloat(Integer) (Variables|Default|GetBlockSize))) Shift)))

(fn CalcShiftbyExtraSize
  (params (ExtraSize :type Vector))
  (bind _blocksize (Variables|Default|GetBlockSize))
  (bind _returnvalue (* _blocksize 2))
  (bind _returnvalue_2 (Math|Conversions|ToFloat(Integer) _returnvalue))
  (return (/ (Math|Vector|MakeVector (Math|Float|%(Float) (.x ExtraSize) _returnvalue_2) (Math|Float|%(Float) (.y ExtraSize) _returnvalue_2) (Math|Float|%(Float) (.z ExtraSize) _returnvalue_2)) (Class|KismetSystemLibrary|MakeLiteralInteger 2))))

(fn GetLoactionforPlacebyPlayer
  (params (Player :type BP%20Player%20Character%20Object%20Reference))
  (bind _crosshairhitresult (Variables|/Game/MAIN_GAME/Blueprints/Player/BP_PlayerCharacter.BP_PlayerCharacter_C|GetCrosshairHitResult Player))
  (bind _returnvalue (- (.traceend _crosshairhitresult) (.tracestart _crosshairhitresult)))
  (bind _itemstruct (Default|GetHandsItemStructPlaceable Player))
  (if (Utilities|Operators|EqualEqual :A (.extrasize _itemstruct))
    (return (CallFunction|SnapLocationtoGrid (.location _crosshairhitresult) (CallFunction|CalcShiftbyExtraSize (.extrasize _itemstruct))))
    (else
      (return (+ (CallFunction|SnapLocationtoGrid (.location _crosshairhitresult) (CallFunction|CalcShiftbyExtraSize (.extrasize _itemstruct))) (* (.normal _crosshairhitresult) (.impactnormal _crosshairhitresult) (/ _returnvalue (Math|Vector|VectorGetAbs _returnvalue)) (Variables|Default|GetBlockSize) (Class|KismetSystemLibrary|MakeLiteralInteger -1)))))))