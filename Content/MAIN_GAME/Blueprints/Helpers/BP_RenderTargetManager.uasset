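; BP_RenderTargetManager is a helper actor that spawns a mesh renderer actor for every item in the DT_Items data table when play begins.
; Each row supplies its own MeshRenderer class, spawned with the manager as owner.
; The renderers are placed very high above the world and spaced along X by a running offset, keeping them apart and away from the playable level.
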(event EventBeginPlay
  (CallFunction|SpawnRenderers))

(fn ConstructionScript)

(fn SpawnRenderers
  (bind _outrownames (DataTable|GetDataTableRowNames "/Game/MAIN_GAME/Data/Items/DT_Items.DT_Items"))
  (for _array_element _outrownames
    (bind _returnvalue (Utilities|GetDataTableRow "/Game/MAIN_GAME/Data/Items/DT_Items.DT_Items" _array_element)
      (:then
        (Game|SpawnActorfromClass (.MeshRenderer (Utilities|Struct|BreakS_Item _returnvalue)) (Math|Transform|MakeTransform (Math|Vector|MakeVector (LocalVariables|GetL_Location) 0.0 1e+07) "0, 0, 0" "1.000000,1.000000,1.000000") "Undefined" self 0)
        (LocalVariables|SetL_Location (+ (LocalVariables|GetL_Location) 5e+01))))))