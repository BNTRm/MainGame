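; BP_Item_Dropped is a dropped world item with a spinning, physics-simulated mesh, a rarity-colored beam and a timed lifespan.
; After a short delay it becomes pickupable and tries adding itself to an overlapping player's inventory through PickUp, expiring on success.
; Overlapping drops with the same stackable ItemId merge by summing quantities, destroying the other actor and showing a stack mesh.
; DT_Items supplies stackability and rarity, with beam color resolved through BP_GameMode.
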(event OnComponentBeginOverlap(ItemCollision)
  (params (OverlappedComponent :type Primitive%20Component%20Object%20Reference) (OtherActor :type Actor%20Object%20Reference) (OtherComp :type Primitive%20Component%20Object%20Reference) (OtherBodyIndex :type Integer) (bFromSweep :type Boolean) (SweepResult :type Hit%20Result%20Structure%20%28by%20ref%29))
  (bind _bp_itemdatacomponent (Variables|Default|GetBP_ItemDataComponent))
  (bind _itemid (Variables|/Game/MAIN_GAME/Blueprints/Items/BP_ItemDataComponent.BP_ItemDataComponent_C|GetItemId _bp_itemdatacomponent))
  (if (!= self OtherActor)
    (bind _asbp_item_dropped (Utilities|Casting|CastToBP_Item_Dropped OtherActor))
    (if (== (Variables|/Game/MAIN_GAME/Blueprints/Items/BP_ItemDataComponent.BP_ItemDataComponent_C|GetItemId (Variables|BP_Item_Dropped_C|GetBP_ItemDataComponent _asbp_item_dropped)) _itemid)
      (bind _returnvalue (Utilities|GetDataTableRow "/Game/MAIN_GAME/Data/Items/DT_Items.DT_Items" _itemid)
        (:then
          (if (> (.MaxStack (Utilities|Struct|BreakS_Item _returnvalue)) 1)
            (CallFunction|ToStack (+ (Variables|/Game/MAIN_GAME/Blueprints/Items/BP_ItemDataComponent.BP_ItemDataComponent_C|GetQuantity (Variables|BP_Item_Dropped_C|GetBP_ItemDataComponent _asbp_item_dropped)) (Variables|/Game/MAIN_GAME/Blueprints/Items/BP_ItemDataComponent.BP_ItemDataComponent_C|GetQuantity _bp_itemdatacomponent)))
            (Actor|DestroyActor OtherActor)))))))

(event Custom|MakeTempNonPickapable
  (params (Seconds :type Float%20%28double-precision%29))
  (Utilities|FlowControl|RetriggerableDelay Seconds)
  (Variables|Default|SetIsPickupable true)
  (CallFunction|PickUpbyPlayerifOverlap))

(event EventBeginPlay
  (bind _staticmesh_stack (Variables|Default|GetStaticMesh_Stack))
  (bind _staticmesh (Variables|Default|GetStaticMesh))
  (Components|StaticMesh|SetStaticMesh _staticmesh_stack (Variables|/Script/Engine.StaticMeshComponent|GetStaticMesh _staticmesh))
  (Rendering|Material|SetMaterial _staticmesh_stack 0 (Rendering|Material|GetMaterial _staticmesh 0))
  (Physics|SetSimulatePhysics (Variables|Default|GetStaticMesh) true)
  (Actor|SetLifeSpan 6e+02)
  (CallFunction|MakeTempNonPickapable 3.0)
  (CallFunction|UpdateRarityBeam))

(event EventTick
  (params (DeltaSeconds :type Float%20%28single-precision%29))
  (Transformation|AddWorldRotation (Variables|Default|GetStaticMesh) "0,1.000000, 0" false false))

(fn ConstructionScript)

(fn PickUp
  (params (Pickuper :type BP%20Player%20Character%20Object%20Reference))
  (bind _bp_itemdatacomponent (Variables|Default|GetBP_ItemDataComponent))
  (bind _bp_inventorycomponent (Variables|/Game/MAIN_GAME/Blueprints/Player/BP_PlayerCharacter.BP_PlayerCharacter_C|GetBP_InventoryComponent Pickuper))
  (if (Variables|Default|GetIsPickupable)
    (Utilities|IsValid _bp_inventorycomponent
      (:Is%20Valid
        (Utilities|IsValid _bp_itemdatacomponent
          (:Is%20Valid
            (bind _success (Default|AddItem _bp_inventorycomponent (Default|GetasSlotItemStruct _bp_itemdatacomponent)))
            (if _success
              (Default|MCUpdate _bp_inventorycomponent)
              (Development|SetHiddeninGame (Variables|Default|GetItemCollision) true true)
              (Components|Activation|Deactivate (Variables|Default|GetItemCollision))
              (Actor|SetLifeSpan 0.1))))))))

(fn ToStack
  (params (Amount :type Integer))
  (Variables|/Game/MAIN_GAME/Blueprints/Items/BP_ItemDataComponent.BP_ItemDataComponent_C|SetQuantity (Variables|Default|GetBP_ItemDataComponent) Amount)
  (Rendering|SetVisibility (Variables|Default|GetStaticMesh_Stack) true false))

(fn PickUpbyPlayerifOverlap
  (bind _itemcollision (Variables|Default|GetItemCollision))
  (Utilities|IsValid _itemcollision
    (:Is%20Valid
      (bind _array_element (Utilities|Array|ForEachLoopwithBreak (Collision|GetOverlappingActors _itemcollision "/Game/MAIN_GAME/Blueprints/Player/BP_PlayerCharacter.BP_PlayerCharacter_C" :!class /Script/Engine.PrimitiveComponent) :!label _label)
        (:LoopBody
          (CallFunction|PickUp (.AsBP%20Player%20Character (Utilities|Casting|CastToBP_PlayerCharacter _array_element)))
          (goto _label Break))))))

(fn UpdateRarityBeam
  (bind _returnvalue (Utilities|GetDataTableRow "/Game/MAIN_GAME/Data/Items/DT_Items.DT_Items" (Variables|/Game/MAIN_GAME/Blueprints/Items/BP_ItemDataComponent.BP_ItemDataComponent_C|GetItemId (Variables|Default|GetBP_ItemDataComponent)))
    (:then
      (Rendering|Material|SetVectorParameterValueonMaterials (Variables|Default|GetRarityBeam) "Color" (Math|Conversions|ToVector(LinearColor) (.specifiedcolor (Default|GetColorbyRarityEnum (.AsBP%20Game%20Mode (Utilities|Casting|CastToBP_GameMode (Game|GetGameMode))) (.Rarity (Utilities|Struct|BreakS_Item _returnvalue)))))))))