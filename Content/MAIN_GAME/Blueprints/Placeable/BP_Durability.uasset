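; BP_Durability is a component that gives its owning actor, likely a placeable, a durability pool that damage can deplete.
; It fills the pool on BeginPlay, subtracts incoming damage in TakeDamage, and destroys the owner at zero or below.
; A retriggerable delay restarts on each non-lethal hit, so durability snaps back to maximum once five seconds pass without further damage.
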(event Custom|TakeDamage
  (params (Damage :type Integer))
  (bind _output_get (Variables|Default|SetCurrentDurability (- (Variables|Default|GetCurrentDurability) Damage)))
  (if (<= _output_get 0)
    (Actor|DestroyActor (Components|GetOwner))
    (else
      (Utilities|FlowControl|RetriggerableDelay 5.0)
      (Variables|Default|SetCurrentDurability (Variables|Default|GetMaxDurability)))))

(event EventBeginPlay
  (Variables|Default|SetCurrentDurability (Variables|Default|GetMaxDurability)))