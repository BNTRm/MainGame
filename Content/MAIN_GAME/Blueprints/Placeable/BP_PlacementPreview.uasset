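; BP_PlacementPreview is the preview actor for placing placeables, showing whether the current spot is valid.
; It counts overlaps between a slightly shrunk collision copy of the mesh and other BP_Placeable actors.
; Any overlap switches the visible mesh to the invalid material, and a zero count restores the valid one.
; IsValid reports that state, and SetStaticMesh applies a given mesh to both components.
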(event OnComponentBeginOverlap(StaticMesh_Collision)
  (params (OverlappedComponent :type Primitive%20Component%20Object%20Reference) (OtherActor :type Actor%20Object%20Reference) (OtherComp :type Primitive%20Component%20Object%20Reference) (OtherBodyIndex :type Integer) (bFromSweep :type Boolean) (SweepResult :type Hit%20Result%20Structure%20%28by%20ref%29))
  (Utilities|Casting|CastToBP_Placeable OtherActor)
  (Math|Integer|IncrementInt (Variables|Default|GetOverlappingCount)
    (:%20%20
      (CallFunction|SetIsValid false))))

(event OnComponentEndOverlap(StaticMesh_Collision)
  (params (OverlappedComponent :type Primitive%20Component%20Object%20Reference) (OtherActor :type Actor%20Object%20Reference) (OtherComp :type Primitive%20Component%20Object%20Reference) (OtherBodyIndex :type Integer))
  (bind _overlappingcount (Variables|Default|GetOverlappingCount))
  (Utilities|Casting|CastToBP_Placeable OtherActor)
  (Math|Integer|DecrementInt _overlappingcount
    (:%20%20
      (if (== _overlappingcount 0)
        (CallFunction|SetIsValid true)))))

(event EventBeginPlay
  (Transformation|SetWorldScale3D (Variables|Default|GetStaticMesh_Collision) "0.970000,0.960000,0.960000"))

(event EventTick
  (params (DeltaSeconds :type Float%20%28single-precision%29)))

(fn ConstructionScript)

(fn SetIsValid
  (params (IsValid :type Boolean))
  (bind _staticmesh (Variables|Default|GetStaticMesh))
  (if IsValid
    (Rendering|Material|SetMaterial _staticmesh 0 (Variables|Default|GetValidMaterial))
    (else
      (Rendering|Material|SetMaterial _staticmesh 0 (Variables|Default|GetInvalidMaterial)))))

(fn IsValid
  (if (== (Variables|Default|GetOverlappingCount) 0)
    (return true)
    (else
      (return false))))

(fn SetStaticMesh
  (params (NewMesh :type Static%20Mesh%20Object%20Reference))
  (Components|StaticMesh|SetStaticMesh (Variables|Default|GetStaticMesh) NewMesh)
  (Components|StaticMesh|SetStaticMesh (Variables|Default|GetStaticMesh_Collision) NewMesh))