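; BP_DragDropComponent handles dragging items between inventory slots in the inventory UI.
; It caches the HUD's drag preview widget shortly after BeginPlay, and StartDrag stores the source slot and shows the item's DT_Items icon at the cursor.
; StopDrag asks the destination inventory to transfer the slots, requiring a matching slot type for equipment components, then clears and hides the preview.
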(event EventBeginPlay
  (Utilities|FlowControl|Delay 0.5)
  (Variables|Default|SetDragPreview (Variables|/Game/MAIN_GAME/UI/WB_PlayerHud.WB_PlayerHud_C|GetWB_DragPreview (Variables|/Game/MAIN_GAME/Player/Blueprints/BP_PlayerController.BP_PlayerController_C|GetPlayerHudWidget (.AsBP%20Player%20Controller (Utilities|Casting|CastToBP_PlayerController (Game|GetPlayerController 0)))))))

(fn StartDrag
  (params (SourceSlot :type WB%20Inventory%20Slot%20Object%20Reference))
  (bind _dragpreview (Variables|Default|GetDragPreview))
  (bind _output_get (Variables|/Game/MAIN_GAME/InventorySystem/Widgets/WB_DragPreview.WB_DragPreview_C|SetInventorySlotWidget (Variables|Default|GetDragPreview) SourceSlot))
  (bind _returnvalue (Utilities|GetDataTableRow "/Game/MAIN_GAME/Items/DT_Items.DT_Items" (.ItemId (Utilities|Struct|BreakS_SlotItem (Variables|/Game/MAIN_GAME/InventorySystem/Widgets/WB_InventorySlot.WB_InventorySlot_C|GetSlotItemStruct _output_get))))
    (:then
      (Appearance|SetBrushfromTexture (Variables|/Game/MAIN_GAME/InventorySystem/Widgets/WB_DragPreview.WB_DragPreview_C|GetImage_Circle (Variables|Default|GetDragPreview)) (.Icon (Utilities|Struct|BreakS_Item _returnvalue)) false)
      (Default|PositiontoMouseCursor _dragpreview)
      (Widget|SetVisibility _dragpreview "Visible"))))

(fn StopDrag
  (params (DestinationSlot :type WB%20Inventory%20Slot%20Object%20Reference))
  (bind _dragpreview (Variables|Default|GetDragPreview))
  (Utilities|IsValid DestinationSlot
    (:Is%20Valid
      (Utilities|IsValid (Variables|/Game/MAIN_GAME/InventorySystem/Widgets/WB_InventorySlot.WB_InventorySlot_C|GetInventoryComponent DestinationSlot)
        (:Is%20Valid
          (Utilities|IsValid (Variables|/Game/MAIN_GAME/InventorySystem/Widgets/WB_InventorySlot.WB_InventorySlot_C|GetInventoryComponent (Variables|/Game/MAIN_GAME/InventorySystem/Widgets/WB_DragPreview.WB_DragPreview_C|GetInventorySlotWidget (Variables|Default|GetDragPreview)))
            (:Is%20Valid
              (bind _returnvalue (Utilities|GetDataTableRow "/Game/MAIN_GAME/Items/DT_Items.DT_Items" (.itemid (Variables|/Game/MAIN_GAME/InventorySystem/Widgets/WB_InventorySlot.WB_InventorySlot_C|GetSlotItemStruct (Variables|/Game/MAIN_GAME/InventorySystem/Widgets/WB_DragPreview.WB_DragPreview_C|GetInventorySlotWidget (Variables|Default|GetDragPreview)))))
                (:then
                  (if (Utilities|ClassIsChildOf (Utilities|GetClass (Variables|/Game/MAIN_GAME/InventorySystem/Widgets/WB_InventorySlot.WB_InventorySlot_C|GetInventoryComponent DestinationSlot)) "/Game/MAIN_GAME/InventorySystem/BP_EquipmentComponent.BP_EquipmentComponent_C")
                    (if (Utilities|Enum|Equal(Enum) (Variables|/Game/MAIN_GAME/InventorySystem/Widgets/WB_InventorySlot.WB_InventorySlot_C|GetType DestinationSlot) (.SlotType (Utilities|Struct|BreakS_Item _returnvalue)))
                      (Default|TransferSlots (Variables|/Game/MAIN_GAME/InventorySystem/Widgets/WB_InventorySlot.WB_InventorySlot_C|GetInventoryComponent DestinationSlot) (Variables|/Game/MAIN_GAME/InventorySystem/Widgets/WB_InventorySlot.WB_InventorySlot_C|GetContent%20Index (Variables|/Game/MAIN_GAME/InventorySystem/Widgets/WB_DragPreview.WB_DragPreview_C|GetInventorySlotWidget (Variables|Default|GetDragPreview))) (Variables|/Game/MAIN_GAME/InventorySystem/Widgets/WB_InventorySlot.WB_InventorySlot_C|GetInventoryComponent (Variables|/Game/MAIN_GAME/InventorySystem/Widgets/WB_DragPreview.WB_DragPreview_C|GetInventorySlotWidget (Variables|Default|GetDragPreview))) (Variables|/Game/MAIN_GAME/InventorySystem/Widgets/WB_InventorySlot.WB_InventorySlot_C|GetContent%20Index DestinationSlot) :!label _label))
                    (else
                      (goto _label))))
                (:RowNotFound
                  _)))
            (:Is%20Not%20Valid
              _)))
        (:Is%20Not%20Valid
          _)))
    (:Is%20Not%20Valid
      _))
  (Variables|/Game/MAIN_GAME/InventorySystem/Widgets/WB_DragPreview.WB_DragPreview_C|SetInventorySlotWidget _dragpreview 0)
  (Widget|SetVisibility _dragpreview "Hidden"))