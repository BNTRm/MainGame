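; Inventory component for the player and other holders, storing items as a fixed-size array of slots sized on BeginPlay.
; AddItem fills matching stacks up to the max stack from DT_Items, then empty slots; RemoveItem and SwapItem are empty stubs.
; Server-side slot transfers swap or merge stacks between inventories, then multicast an update to both.
; It also routes interact input to the server, which interacts with item actors or hands ownership and a local interact to others.
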(event Custom|MC_Update
  (Default|CallOnInventoryUpdated))

(event Custom|Server_Intearct
  (params (Target :type Actor%20Object%20Reference) (Interactor :type BP%20Player%20Character%20Object%20Reference))
  (Utilities|IsValid Target
    (:Is%20Valid
      (Utilities|IsValid (Actor|GetComponentbyClass Target "/Game/MAIN_GAME/Items/BP_ItemDataComponent.BP_ItemDataComponent_C")
        (:Is%20Valid
          (Class|BPIInteractable|Interactwith(Message) Target Interactor))
        (:Is%20Not%20Valid
          (Actor|SetOwner Target (Pawn|GetController Interactor))
          (CallFunction|OnLocalInteract Target Interactor))))))

(event Custom|Server_TransferSlots
  (params (SourceIndex :type Integer) (SourceInventory :type BP%20Inventory%20Component%20Object%20Reference) (DestinationIndex :type Integer))
  (CallFunction|TransferSlots SourceIndex SourceInventory DestinationIndex))

(event Custom|OnLocalInteract
  (params (Target :type Actor%20Object%20Reference) (Interactor :type Actor%20Object%20Reference))
  (Class|BPIInteractable|Interactwith(Message) Target (.AsBP%20Player%20Character (Utilities|Casting|CastToBP_PlayerCharacter Interactor))))

(event EventBeginPlay
  (Utilities|Array|Resize (Variables|Default|GetItems) (Variables|Default|GetSize)))

(event Input|ActionEvents|InputActionInteract/AltFire/Place
  (params (Key :type Key%20Structure :default "None"))
  (bind _returnvalue (Components|GetOwner))
  (bind _asbp_player_character (Utilities|Casting|CastToBP_PlayerCharacter _returnvalue))
  (:Pressed
    (CallFunction|ServerIntearct (Variables|/Game/MAIN_GAME/Player/Blueprints/BP_PlayerCharacter.BP_PlayerCharacter_C|GetInteractableActor _asbp_player_character) _asbp_player_character)))

(fn AddItem
  (params (ItemSlotStruct :type S%20Slot%20Item%20Structure))
  (LocalVariables|SetL_QuantityRemaining (.quantity ItemSlotStruct))
  (while (and (> (LocalVariables|GetL_QuantityRemaining) 0) (not (LocalVariables|GetL_IsFailed)))
    (bind (_index _isslotfound) (CallFunction|FindSlot (.itemid ItemSlotStruct)))
    (if _isslotfound
      (CallFunction|AddtoStack _index 1)
      (Math|Integer|DecrementInt (LocalVariables|GetL_QuantityRemaining))
      (elif (.HasEmptySlot (CallFunction|AnyEmptySlotsAvailable))
        (bind _success (CallFunction|CreateNewStack (Utilities|Struct|MakeS_SlotItem (.itemid ItemSlotStruct) 1)))
        (if _success
          (Math|Integer|DecrementInt (LocalVariables|GetL_QuantityRemaining))
          (else
            (LocalVariables|SetL_IsFailed true)))
        (else
          (LocalVariables|SetL_IsFailed true)))))
  (return (not (LocalVariables|GetL_IsFailed)) (LocalVariables|GetL_QuantityRemaining)))

(fn AddtoStack
  (params (Index :type Integer) (Quantity :type Integer))
  (bind _items (Variables|Default|GetItems))
  (bind _output (Utilities|Array|Get(acopy) _items Index))
  (Utilities|Array|SetArrayElem (Variables|Default|GetItems) Index (Utilities|Struct|MakeS_SlotItem (.itemid _output) (+ (.quantity _output) Quantity))))

(fn AnyEmptySlotsAvailable
  (for (_array_element _array_index) (Variables|Default|GetItems)
    (if (== (.Quantity (Utilities|Struct|BreakS_SlotItem _array_element)) 0)
      (return true _array_index)))
  (return false -1))

(fn CreateNewStack
  (params (ItemSlotStruct :type S%20Slot%20Item%20Structure))
  (bind (_hasemptyslot _emptyslotindex) (CallFunction|AnyEmptySlotsAvailable))
  (if _hasemptyslot
    (Utilities|Array|SetArrayElem (Variables|Default|GetItems) _emptyslotindex ItemSlotStruct)
    (return true)
    (else
      (return false))))

(fn FindSlot
  (params (ItemID :type Name))
  (for (_array_element _array_index) (Variables|Default|GetItems)
    (if (== (.ItemId (Utilities|Struct|BreakS_SlotItem _array_element)) ItemID)
      (if (< (.Quantity (Utilities|Struct|BreakS_SlotItem _array_element)) (CallFunction|GetItemMaxStack ItemID))
        (return _array_index true))))
  (return -1 false))

(fn GetItemMaxStack
  (params (ItemID :type Name))
  (bind _returnvalue (Utilities|GetDataTableRow "/Game/MAIN_GAME/Data/Items/DT_Items.DT_Items" ItemID)
    (:then
      (return (.maxstack _returnvalue)))
    (:RowNotFound
      (return -1))))

(fn RemoveItem)

(fn SwapItem)

(fn TransferSlots
  (params (SourceIndex :type Integer) (SourceInventory :type BP%20Inventory%20Component%20Object%20Reference) (DestinationIndex :type Integer))
  (LocalVariables|SetL_SourceSlotContent (Utilities|Array|Get(acopy) (Variables|BP_InventoryComponent_C|GetItems SourceInventory) SourceIndex))
  (if (not (< DestinationIndex 0))
    (if (!= (.itemid (LocalVariables|GetL_SourceSlotContent)) (.itemid (Utilities|Array|Get(acopy) (Variables|Default|GetItems) DestinationIndex)))
      ;[1 1 1] Swap (Different Items)
      (Utilities|Array|SetArrayElem (Variables|BP_InventoryComponent_C|GetItems SourceInventory) SourceIndex (Utilities|Array|Get(acopy) (Variables|Default|GetItems) DestinationIndex))
      (Utilities|Array|SetArrayElem (Variables|Default|GetItems) DestinationIndex (LocalVariables|GetL_SourceSlotContent))
      (else
        ;[1 1 1] Stack (Same Items)
        (Utilities|Array|SetArrayElem (Variables|BP_InventoryComponent_C|GetItems SourceInventory) SourceIndex (Utilities|Struct|MakeS_SlotItem (select (> (Math|Integer|Clamp(Integer) (- (+ (.quantity (LocalVariables|GetL_SourceSlotContent)) (.quantity (Utilities|Array|Get(acopy) (Variables|Default|GetItems) DestinationIndex))) (CallFunction|GetItemMaxStack (.itemid (LocalVariables|GetL_SourceSlotContent)))) 0 (CallFunction|GetItemMaxStack (.itemid (LocalVariables|GetL_SourceSlotContent)))) 0) (.itemid (LocalVariables|GetL_SourceSlotContent)) "None") (Math|Integer|Clamp(Integer) (- (+ (.quantity (LocalVariables|GetL_SourceSlotContent)) (.quantity (Utilities|Array|Get(acopy) (Variables|Default|GetItems) DestinationIndex))) (CallFunction|GetItemMaxStack (.itemid (LocalVariables|GetL_SourceSlotContent)))) 0 (CallFunction|GetItemMaxStack (.itemid (LocalVariables|GetL_SourceSlotContent))))))
        (Utilities|Array|SetArrayElem (Variables|Default|GetItems) DestinationIndex (Utilities|Struct|MakeS_SlotItem (.itemid (LocalVariables|GetL_SourceSlotContent)) (Math|Integer|Clamp(Integer) (+ (.quantity (LocalVariables|GetL_SourceSlotContent)) (.quantity (Utilities|Array|Get(acopy) (Variables|Default|GetItems) DestinationIndex))) 0 (CallFunction|GetItemMaxStack (.itemid (LocalVariables|GetL_SourceSlotContent))))))))
    (CallFunction|MCUpdate)
    (CallFunction|MCUpdate SourceInventory)))