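; Player equipment component that shows equipped items as actors attached to the player character.
; On BeginPlay it caches the owning BP_PlayerCharacter and binds to inventory updates.
; UpdateEquipmentFull destroys and respawns head, body, arms, legs and feet items, attaching each to its socket and hiding hair under headgear.
; UpdateEquipmentElement spawns each actor class by looking up the slot's item ID in DT_Items_Equipment.
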(event EventBeginPlay
  (|CallParentFunction)
  (Variables|Default|SetPlayerCharacter (.AsBP%20Player%20Character (Utilities|Casting|CastToBP_PlayerCharacter (Components|GetOwner))))
  (EventDispatchers|BindEventtoOnInventoryUpdated (EventDispatchers|CreateEvent :!event UpdateEquipmentFull)))

(fn UpdateEquipmentElement
  (params (ItemIndex :type Integer))
  (bind _output (CallFunction|GetSlotItemStructbyIndex ItemIndex))
  (bind _returnvalue (Utilities|GetDataTableRow "/Game/MAIN_GAME/Data/Items/DT_Items_Equipment.DT_Items_Equipment" (.itemid _output))
    (:then
      (bind _returnvalue_2 (Game|SpawnActorfromClass (.equipped_bpclass _returnvalue) (Math|Transform|MakeTransform (Transformation|GetActorLocation (Variables|Default|GetPlayerCharacter)) "0, 0, 0" "1.000000,1.000000,1.000000") "Undefined" 0 0))
      (return _returnvalue_2))
    (:RowNotFound
      (return 0))))

(fn UpdateEquipmentFull
  (bind _playercharacter (Variables|Default|GetPlayerCharacter))
  (Utilities|FlowControl|Sequence
    (:then_0
      (Utilities|IsValid (Variables|Default|GetEquippedItem_Head)
        (:Is%20Valid
          (Actor|DestroyActor (Variables|Default|GetEquippedItem_Head)))
        (:Is%20Not%20Valid
          _))
      (bind _returnvalue (CallFunction|UpdateEquipmentElement (Variables|Default|GetHeadIndex)))
      (Utilities|IsValid _returnvalue
        (:Is%20Valid
          (Default|SetHairVisible _playercharacter false)
          (bind _output_get (Variables|Default|SetEquippedItem_Head _returnvalue))
          (Default|AttachEquipItem (Variables|Default|GetPlayerCharacter) _output_get "Socket_Head"))
        (:Is%20Not%20Valid
          (Default|SetHairVisible _playercharacter true))))
    (:then_1
      (Utilities|IsValid (Variables|Default|GetEquippedItem_Body)
        (:Is%20Valid
          (Actor|DestroyActor (Variables|Default|GetEquippedItem_Body)))
        (:Is%20Not%20Valid
          _))
      (bind _returnvalue_2 (CallFunction|UpdateEquipmentElement (Variables|Default|GetBodyIndex)))
      (Utilities|IsValid _returnvalue_2
        (:Is%20Valid
          (bind _output_get_2 (Variables|Default|SetEquippedItem_Body _returnvalue_2))
          (Default|AttachEquipItem (Variables|Default|GetPlayerCharacter) _output_get_2 "Socket_Body"))))
    (:then_2
      (Utilities|IsValid (Variables|Default|GetEquippedItem_Arms)
        (:Is%20Valid
          (Actor|DestroyActor (Variables|Default|GetEquippedItem_Arms)))
        (:Is%20Not%20Valid
          _))
      (bind _returnvalue_3 (CallFunction|UpdateEquipmentElement (Variables|Default|GetArmsIndex)))
      (Utilities|IsValid _returnvalue_3
        (:Is%20Valid
          (bind _output_get_3 (Variables|Default|SetEquippedItem_Arms _returnvalue_3))
          (Default|AttachEquipItem (Variables|Default|GetPlayerCharacter) _output_get_3 "Socket_Arms"))))
    (:then_3
      (Utilities|IsValid (Variables|Default|GetEquippedItem_Legs)
        (:Is%20Valid
          (Actor|DestroyActor (Variables|Default|GetEquippedItem_Legs)))
        (:Is%20Not%20Valid
          _))
      (bind _returnvalue_4 (CallFunction|UpdateEquipmentElement (Variables|Default|GetLegsIndex)))
      (Utilities|IsValid _returnvalue_4
        (:Is%20Valid
          (bind _output_get_4 (Variables|Default|SetEquippedItem_Legs _returnvalue_4))
          (Default|AttachEquipItem (Variables|Default|GetPlayerCharacter) _output_get_4 "Socket_Legs"))))
    (:then_4
      (Utilities|IsValid (Variables|Default|GetEquippedItem_Feet)
        (:Is%20Valid
          (Actor|DestroyActor (Variables|Default|GetEquippedItem_Feet)))
        (:Is%20Not%20Valid
          _))
      (bind _returnvalue_5 (CallFunction|UpdateEquipmentElement (Variables|Default|GetFeetIndex)))
      (Utilities|IsValid _returnvalue_5
        (:Is%20Valid
          (bind _output_get_5 (Variables|Default|SetEquippedItem_Feet _returnvalue_5))
          (Default|AttachEquipItem (Variables|Default|GetPlayerCharacter) _output_get_5 "Socket_Feet"))))))