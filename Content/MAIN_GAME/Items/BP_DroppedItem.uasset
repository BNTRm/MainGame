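; BP_DroppedItem is a world item the player can look at and pick up into their inventory.
; PickUp adds the item data component's slot struct to the player character's inventory component and destroys the actor only if the add succeeds.
; LookAt looks up the item ID in DT_Items and returns a "Pick up" prompt with the item's name.
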(event Custom|PickUp
  (params (Puckuper :type Character%20Object%20Reference))
  (bind _asbp_player_character (Utilities|Casting|CastToBP_PlayerCharacter Puckuper))
  (bind _bp_itemdatacomponent (Variables|Default|GetBP_ItemDataComponent))
  (bind _bp_inventorycomponent (Variables|/Game/MAIN_GAME/Player/Blueprints/BP_PlayerCharacter.BP_PlayerCharacter_C|GetBP_InventoryComponent _asbp_player_character))
  (Utilities|IsValid _bp_inventorycomponent
    (:Is%20Valid
      (Utilities|IsValid _bp_itemdatacomponent
        (:Is%20Valid
          (bind _success (Default|AddItem _bp_inventorycomponent (Variables|/Game/MAIN_GAME/Items/BP_ItemDataComponent.BP_ItemDataComponent_C|GetSlotItemStruct _bp_itemdatacomponent)))
          (if _success
            (Actor|DestroyActor)))))))

(event EventBeginPlay)

(event Collision|EventActorBeginOverlap
  (params (OtherActor :type Actor%20Object%20Reference)))

(event EventTick
  (params (DeltaSeconds :type Float%20%28single-precision%29)))

(fn ConstructionScript)

(fn Lookat
  (params (Observer :type Voxman%20Character%20Object%20Reference))
  (bind _returnvalue (Utilities|GetDataTableRow "/Game/MAIN_GAME/Data/Items/DT_Items.DT_Items" (.itemid (Variables|/Game/MAIN_GAME/Items/BP_ItemDataComponent.BP_ItemDataComponent_C|GetSlotItemStruct (Variables|Default|GetBP_ItemDataComponent))))
    (:then
      (return (Utilities|Text|FormatText "Pick up {item}" (.Name (Utilities|Struct|BreakS_Item _returnvalue))) "None"))))