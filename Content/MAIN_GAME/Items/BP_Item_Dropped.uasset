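; Dropped world item that simulates physics, slowly spins, expires after a timed lifespan and can be picked up into a player's inventory.
; After a short delay it becomes pickupable and goes to an already overlapping player; PickUp destroys it once the inventory accepts it.
; Overlapping drops with the same stackable DT_Items ID merge quantities into one actor, revealing a second stack mesh.
; LookAt supplies the named "Pick up" prompt.
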(event OnComponentBeginOverlap(ItemCollision)
  (params (OverlappedComponent :type Primitive%20Component%20Object%20Reference) (OtherActor :type Actor%20Object%20Reference) (OtherComp :type Primitive%20Component%20Object%20Reference) (OtherBodyIndex :type Integer) (bFromSweep :type Boolean) (SweepResult :type Hit%20Result%20Structure%20%28by%20ref%29))
  (bind _bp_itemdatacomponent (Variables|Default|GetBP_ItemDataComponent))
  (bind _itemid (Variables|/Game/MAIN_GAME/Items/BP_ItemDataComponent.BP_ItemDataComponent_C|GetItemId _bp_itemdatacomponent))
  (if (!= OtherActor self)
    (bind _asbp_item_dropped (Utilities|Casting|CastToBP_Item_Dropped OtherActor))
    (if (== (Variables|/Game/MAIN_GAME/Items/BP_ItemDataComponent.BP_ItemDataComponent_C|GetItemId (Variables|BP_Item_Dropped_C|GetBP_ItemDataComponent _asbp_item_dropped)) _itemid)
      (bind _returnvalue (Utilities|GetDataTableRow "/Game/MAIN_GAME/Items/DT_Items.DT_Items" _itemid)
        (:then
          (if (.stackable _returnvalue)
            (CallFunction|ToStack (+ (Variables|/Game/MAIN_GAME/Items/BP_ItemDataComponent.BP_ItemDataComponent_C|GetQuantity (Variables|BP_Item_Dropped_C|GetBP_ItemDataComponent _asbp_item_dropped)) (Variables|/Game/MAIN_GAME/Items/BP_ItemDataComponent.BP_ItemDataComponent_C|GetQuantity _bp_itemdatacomponent)))
            (Actor|DestroyActor OtherActor)))))))

(event Custom|PickUp
  (params (Pickuper :type Character%20Object%20Reference))
  (bind _asbp_player_character (Utilities|Casting|CastToBP_PlayerCharacter Pickuper))
  (bind _bp_itemdatacomponent (Variables|Default|GetBP_ItemDataComponent))
  (bind _bp_inventorycomponent (Variables|/Game/MAIN_GAME/Player/Blueprints/BP_PlayerCharacter.BP_PlayerCharacter_C|GetBP_InventoryComponent _asbp_player_character))
  (if (Variables|Default|GetIsPickupable)
    (Utilities|IsValid _bp_inventorycomponent
      (:Is%20Valid
        (Utilities|IsValid _bp_itemdatacomponent
          (:Is%20Valid
            (bind _success (Default|AddItem _bp_inventorycomponent (Default|GetasSlotItemStruct _bp_itemdatacomponent)))
            (if _success
              (Default|MCUpdate _bp_inventorycomponent)
              (Actor|DestroyActor))))))))

(event Custom|ToStack
  (params (Amount :type Integer))
  (Variables|/Game/MAIN_GAME/Items/BP_ItemDataComponent.BP_ItemDataComponent_C|SetQuantity (Variables|Default|GetBP_ItemDataComponent) Amount)
  (Rendering|SetVisibility (Variables|Default|GetStaticMesh_Stack) true false))

(event Custom|ToSingle
  (Variables|/Game/MAIN_GAME/Items/BP_ItemDataComponent.BP_ItemDataComponent_C|SetQuantity (Variables|Default|GetBP_ItemDataComponent) 1)
  (Rendering|SetVisibility (Variables|Default|GetStaticMesh_Stack) false false))

(event EventBeginPlay
  (bind _staticmesh_stack (Variables|Default|GetStaticMesh_Stack))
  (bind _staticmesh (Variables|Default|GetStaticMesh))
  (Components|StaticMesh|SetStaticMesh _staticmesh_stack (Variables|/Script/Engine.StaticMeshComponent|GetStaticMesh _staticmesh))
  (Rendering|Material|SetMaterial _staticmesh_stack 0 (Rendering|Material|GetMaterial _staticmesh 0))
  (Physics|SetSimulatePhysics (Variables|Default|GetStaticMesh) true)
  (Actor|SetLifeSpan 6e+02)
  (Utilities|FlowControl|Delay 2.0)
  (Variables|Default|SetIsPickupable true)
  (bind _array_element (Utilities|Array|ForEachLoopwithBreak (Collision|GetOverlappingActors (Variables|Default|GetItemCollision) "/Game/MAIN_GAME/Player/Blueprints/BP_PlayerCharacter.BP_PlayerCharacter_C" :!class /Script/Engine.PrimitiveComponent) :!label _label)
    (:LoopBody
      (CallFunction|PickUp (.AsBP%20Player%20Character (Utilities|Casting|CastToBP_PlayerCharacter _array_element)))
      (goto _label Break))))

(event EventTick
  (params (DeltaSeconds :type Float%20%28single-precision%29))
  (Transformation|AddWorldRotation (Variables|Default|GetStaticMesh) "0,1.000000, 0" false false))

(fn ConstructionScript)

(fn Lookat
  (params (Observer :type Object%20Object%20Reference))
  (bind _returnvalue (Utilities|GetDataTableRow "/Game/MAIN_GAME/Items/DT_Items.DT_Items" (Variables|/Game/MAIN_GAME/Items/BP_ItemDataComponent.BP_ItemDataComponent_C|GetItemId (Variables|Default|GetBP_ItemDataComponent)))
    (:then
      (return (Utilities|Text|FormatText "Pick up {item}" (.Name (Utilities|Struct|BreakS_Item _returnvalue))) "None"))))