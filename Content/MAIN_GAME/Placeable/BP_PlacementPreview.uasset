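; Placement preview actor that displays a swappable static mesh with a valid or invalid material, for placing objects.
; Every Tick scans the mesh's overlapping actors and sets the invalid material on the first BP_Placeable found, then breaks.
; ToValid follows the loop, so as written it also runs after a break and overrides the invalid material.
; ChangeStaticMesh swaps the previewed mesh.
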(event Custom|ChangeStaticMesh
  (params (NewMesh :type Static%20Mesh%20Object%20Reference))
  (Components|StaticMesh|SetStaticMesh (Variables|Default|GetStaticMesh) NewMesh))

(event Custom|ToValid
  (Rendering|Material|SetMaterial (Variables|Default|GetStaticMesh) 0 (Variables|Default|GetValidMaterial)))

(event Custom|ToInvalid
  (Rendering|Material|SetMaterial (Variables|Default|GetStaticMesh) 0 (Variables|Default|GetInvalidMaterial)))

(event EventBeginPlay)

(event Collision|EventActorBeginOverlap
  (params (OtherActor :type Actor%20Object%20Reference)))

(event EventTick
  (params (DeltaSeconds :type Float%20%28single-precision%29))
  (bind _array_element (Utilities|Array|ForEachLoopwithBreak (Collision|GetOverlappingActors (Variables|Default|GetStaticMesh) 0 :!class /Script/Engine.PrimitiveComponent) :!label _label)
    (:LoopBody
      (Utilities|Casting|CastToBP_Placeable _array_element)
      (CallFunction|ToInvalid)
      (goto _label Break))
    (:Completed
      (CallFunction|ToValid))))

(fn ConstructionScript)