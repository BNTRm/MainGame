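; Player controller that creates the player HUD and routes inventory and hotbar input to it.
; On BeginPlay it creates WB_PlayerHud for the local controller only, stores the widget and adds it to the viewport.
; The Inventory input closes any open menus or opens the inventory menu.
; Next and previous slot inputs change the hotbar selection, refresh the hotbar and call OnHotbarSlotChanged.
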(event EventBeginPlay
  (|DisplayPlayerHud))

(event Input|ActionEvents|InputActionInventory
  (params (Key :type Key%20Structure :default "None"))
  (bind _playerhudwidget (Variables|Default|GetPlayerHudWidget))
  (:Pressed
    (if (Default|IsSomeMenuOpened (Variables|Default|GetPlayerHudWidget))
      (Default|CloseAllMenus _playerhudwidget)
      (else
        (Default|OpenInventoryMenu _playerhudwidget true)))))

(event Input|ActionEvents|InputActionNextHotbarSlot
  (params (Key :type Key%20Structure :default "None"))
  (bind _playerhudwidget (Variables|Default|GetPlayerHudWidget))
  (bind _hotbarwidget (Variables|/Game/MAIN_GAME/UI/WB_PlayerHud.WB_PlayerHud_C|GetHotbarWidget _playerhudwidget))
  (:Pressed
    (Default|SelectNextSlot _hotbarwidget)
    (Default|UpdateHotbar _hotbarwidget)
    (Default|CallOnHotbarSlotChanged)))

(event Input|ActionEvents|InputActionPreviousHotbarSlot
  (params (Key :type Key%20Structure :default "None"))
  (bind _playerhudwidget (Variables|Default|GetPlayerHudWidget))
  (bind _hotbarwidget (Variables|/Game/MAIN_GAME/UI/WB_PlayerHud.WB_PlayerHud_C|GetHotbarWidget _playerhudwidget))
  (:Pressed
    (Default|SelectPreviousSlot _hotbarwidget)
    (Default|UpdateHotbar _hotbarwidget)
    (Default|CallOnHotbarSlotChanged)))

(fn ConstructionScript)