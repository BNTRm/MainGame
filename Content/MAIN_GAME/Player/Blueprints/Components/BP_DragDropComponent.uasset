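; Component that handles inventory drag and drop for the player, including dropping the held item into the world.
; A drag moves the stack into slot 0 of the controller's DragDropInventoryComponent and shows the HUD preview at the cursor.
; Stopping transfers it to the destination, with equipment requiring a matching DT_Items slot type; invalid destinations or unknown items return it to the source.
; Dropping spawns items through the GameMode's DroppedItemsManager with forward impulse.
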(event EventBeginPlay
  (bind _output_get (Variables|Default|SetPlayerController (.AsBP%20Player%20Controller (Utilities|Casting|CastToBP_PlayerController (Game|GetPlayerController 0)))))
  (Variables|Default|SetDragDropInventoryComponent (Variables|/Game/MAIN_GAME/Player/Blueprints/BP_PlayerController.BP_PlayerController_C|GetDragDropInventoryComponent _output_get)))

(fn StartDrag
  (params (SourceIndex :type Integer) (SourceInventory :type BP%20Inventory%20Component%20Object%20Reference))
  (bind _playercontroller (Variables|Default|GetPlayerController))
  (bind _playerhudwidget (Variables|/Game/MAIN_GAME/Player/Blueprints/BP_PlayerController.BP_PlayerController_C|GetPlayerHudWidget _playercontroller))
  (bind _wb_dragpreview (Variables|/Game/MAIN_GAME/UI/WB_PlayerHud.WB_PlayerHud_C|GetWB_DragPreview _playerhudwidget))
  (bind _output_get (Variables|Default|SetDragSourceInventory SourceInventory))
  (bind _output_get_2 (Variables|Default|SetDragSourceIndex SourceIndex))
  (Default|TransferSlots (Variables|Default|GetDragDropInventoryComponent) _output_get_2 _output_get)
  (Default|Update _wb_dragpreview)
  (Default|PositiontoMouseCursor _wb_dragpreview)
  (Widget|SetVisibility _wb_dragpreview "Visible"))

(fn StopDrag
  (params (DestinationInventory :type BP%20Inventory%20Component%20Object%20Reference) (DestinationIndex :type Integer) (DestinationSlotType :type EN_SlotType%20Enum :default "NewEnumerator0"))
  (if (> (.quantity (Default|GetDraggableSlotItem (Variables|Default|GetPlayerController))) 0)
    (Utilities|IsValid DestinationInventory
      (:Is%20Valid
        (bind _returnvalue (Utilities|GetDataTableRow "/Game/MAIN_GAME/Items/DT_Items.DT_Items" (.itemid (Default|GetDraggableSlotItem (Variables|Default|GetPlayerController))))
          (:then
            (if (Default|IsEquipment DestinationInventory)
              (if (Utilities|Enum|Equal(Enum) DestinationSlotType (.slottype _returnvalue))
                (Default|TransferSlots DestinationInventory 0 (Variables|Default|GetDragDropInventoryComponent) DestinationIndex :!label _label)
                (if (> (.quantity (Default|GetDraggableSlotItem (Variables|Default|GetPlayerController))) 0)
                  (Default|Update (Variables|/Game/MAIN_GAME/UI/WB_PlayerHud.WB_PlayerHud_C|GetWB_DragPreview (Variables|/Game/MAIN_GAME/Player/Blueprints/BP_PlayerController.BP_PlayerController_C|GetPlayerHudWidget (Variables|Default|GetPlayerController))))
                  (else
                    (Widget|SetVisibility (Variables|/Game/MAIN_GAME/UI/WB_PlayerHud.WB_PlayerHud_C|GetWB_DragPreview (Variables|/Game/MAIN_GAME/Player/Blueprints/BP_PlayerController.BP_PlayerController_C|GetPlayerHudWidget (Variables|Default|GetPlayerController))) "Hidden" :!label _label_2)
                    (Utilities|Array|SetArrayElem (Variables|/Game/MAIN_GAME/InventorySystem/BP_InventoryComponent.BP_InventoryComponent_C|GetItems (Variables|Default|GetDragDropInventoryComponent)) 0 (Utilities|Struct|MakeS_SlotItem "None")))))
              (else
                (goto _label))))
          (:RowNotFound
            (Default|TransferSlots (Variables|Default|GetDragSourceInventory) 0 (Variables|Default|GetDragDropInventoryComponent) (Variables|Default|GetDragSourceIndex) :!label _label_3)
            (goto _label_2))))
      (:Is%20Not%20Valid
        (goto _label_3)))
    (else
      (goto _label_2))))

(fn DropDraggableItem
  (params (Amount :type Integer))
  (bind _playercontroller (Variables|Default|GetPlayerController))
  (bind _returnvalue (Pawn|GetControlledPawn _playercontroller))
  (bind _asbp_player_character (Utilities|Casting|CastToBP_PlayerCharacter _returnvalue))
  (bind _capsulecomponent (Variables|/Script/Engine.Character|GetCapsuleComponent _asbp_player_character))
  (if (> Amount 0)
    (Default|SpawnDroppedItem (Variables|/Game/MAIN_GAME/Blueprints/BP_GameMode.BP_GameMode_C|GetDroppedItemsManager (.AsBP%20Game%20Mode (Utilities|Casting|CastToBP_GameMode (Game|GetGameMode)))) (Transformation|GetWorldLocation _capsulecomponent) (.itemid (Default|GetDraggableSlotItem (Variables|Default|GetPlayerController))) Amount (* (Math|Vector|GetForwardVector _capsulecomponent) (Math|Float|MakeLiteralFloat 1e+03)))
    (Default|SubtractfromStack (Variables|Default|GetDragDropInventoryComponent) 0 Amount)))